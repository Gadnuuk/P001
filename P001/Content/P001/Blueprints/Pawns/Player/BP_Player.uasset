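; Player character Blueprint that triggers traversal moves, climbing and a fence jump, through its traversal movement component.
; BeginPlay caches the default gravity scale and camera boom length, which this graph does not read back.
; The G key plays the fence jump montage, raising the legs at start and dropping them on completion, blend-out or interruption.
; The TraverseTest input starts climbing; the StopClimbing call is unconnected.
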(event EventBeginPlay
  (Variables|Default|SetDefaultGravityScale (Variables|/Script/Engine.CharacterMovementComponent|GetGravityScale (Variables|Character|GetCharacterMovement)))
  (Variables|Default|SetDefaultCameraBoom (Variables|/Script/Engine.SpringArmComponent|GetTargetArmLength (Variables|Default|GetCameraBoom))))

(event Collision|EventActorBeginOverlap
  (params (OtherActor :type Actor%20Object%20Reference)))

(event EventTick
  (params (DeltaSeconds :type Float%20%28single-precision%29)))

(event Input|ActionEvents|InputActionTraverseTest
  (params (Key :type Key%20Structure :default "None"))
  (:Pressed
    (Class|TraversalMovementComponent|StartClimbing (Class|P001Character|GetTraversalMovementComponent))))

(event Input|KeyboardEvents|G
  (params (Key :type Key%20Structure :default "None"))
  (:Pressed
    (Animation|Montage|PlayMontage (Variables|Character|GetMesh) "/Game/Assets/Mannequin/Animations/UpdatedAnimations/Traversing/Vault/Fence_91cm_JumpOver/Montage_Fence_91cm_JumpOver.Montage_Fence_91cm_JumpOver"
      (:then
        (Class|TraversalMovementComponent|RaiseLegs (Class|P001Character|GetTraversalMovementComponent)))
      (:OnCompleted
        (Class|TraversalMovementComponent|DropLegs (Class|P001Character|GetTraversalMovementComponent) :!label _label))
      (:OnBlendOut
        (goto _label))
      (:OnInterrupted
        (goto _label)))))

(fn ConstructionScript)