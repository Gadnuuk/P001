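; BP_WallPointActor is an interactable wall point that puts the player into a hanging state.
; On interact, it snaps the player in 2D to an offset from GoDownPos toward the actor, preserving lateral offset along the wall using cross-product projection.
; It smoothly yaws the player along the GoDownPos-to-actor direction.
; It also hides the prompt, disables capsule and camera collision, sets Flying movement and switches to BP_HangState.
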(event EventInteract
  (params (player :type BP%20Character%20Object%20Reference))
  (bind _returnvalue (Transformation|GetActorLocation))
  (bind _returnvalue_2 (Transformation|GetActorUpVector))
  (bind _returnvalue_3 (Transformation|GetActorLocation))
  (bind _returnvalue_4 (Transformation|GetActorLocation player))
  (bind _returnvalue_5 (Transformation|GetActorLocation player))
  (bind _godown_pos (Variables|Default|GetGoDown_Pos))
  (bind _returnvalue_6 (Transformation|GetWorldLocation _godown_pos))
  (bind _returnvalue_7 (- _returnvalue_3 _returnvalue_6))
  (bind _returnvalue_8 (Math|Vector|Normalize _returnvalue_7))
  (bind _returnvalue_9 (Math|Vector|CrossProduct _returnvalue_2 _returnvalue_8))
  (Default|UIHideInteractionUI player)
  (Variables|/Script/Engine.SpringArmComponent|SetbDoCollisionTest (Variables|/Game/Assets/AmplifyAnimationPack/Blueprints/Character/BP_Character.BP_Character_C|GetCameraArm player) false)
  (Default|AdjustPosition player _returnvalue_5 (- (+ _returnvalue_6 (* _returnvalue_8 45.0) (* _returnvalue_9 (* (Math|Vector|VectorLength (Math|Vector|ProjectVectorontoVector (- _returnvalue_4 _returnvalue) _returnvalue_9)) (* (Math|Float|Sign(Float) (Math|Vector|DotProduct (Math|Rotator|GetRotationXVector (Math|Rotator|FindLookatRotation _returnvalue_4 _returnvalue)) _returnvalue_9)) -1.0)))) _returnvalue_5) false false true)
  (Default|AdjustRotation player (Math|Rotator|GetRotationXVector (Math|Rotator|MakeRotator 0.0 0.0 (.yaw (Math|Rotator|FindLookatRotation (Transformation|GetWorldLocation (Variables|Default|GetGoDown_Pos)) (Transformation|GetActorLocation))))) true 7.0)
  (Collision|SetCollisionEnabled (Variables|/Script/Engine.Character|GetCapsuleComponent player) "NoCollision")
  (Pawn|Components|CharacterMovement|SetMovementMode (Variables|/Script/Engine.Character|GetCharacterMovement player) "MOVE_Flying" 0)
  (Default|ChangeCurrentState player "/Game/Assets/AmplifyAnimationPack/Blueprints/Character/CharacterStates/BP_HangState.BP_HangState_C"))

(fn ConstructionScript)

(fn CheckResetPlayerCrouch
  (return false))