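; Motorboat variant of a boat interactable that adds visual feedback to the outboard motor while a player character uses it.
; Each tick it yaws the motor mesh from its initial rotation using the Boat_HandTurnAmount animation curve, so the motor follows the character's steering hand.
; Forward input sets the splash particle spawn rate, interpolated toward full when driving, lower when only turning, and zero when idle.
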(event EventTick
  (params (DeltaSeconds :type Float%20%28single-precision%29))
  (bind _playerchar (Variables|Default|GetplayerChar))
  (|CallParentFunction 0.0)
  (Utilities|IsValid _playerchar
    (:Is%20Valid
      (bind _asanim_instance (Utilities|Casting|CastToAnimInstance (Variables|/Game/Assets/AmplifyAnimationPack/Blueprints/Character/BP_Character.BP_Character_C|GetcharAnimCommunicator _playerchar)))
      (Transformation|SetRelativeRotation (Variables|Default|GetMotorMesh) (Math|Rotator|MakeRotator 0.0 0.0 (+ (.yaw (Variables|Default|GetmotorMeshInitialRot)) (* (Animation|Curves|GetCurveValue _asanim_instance "Boat_HandTurnAmount") 2e+01))) false false))))

(event EventBeginPlay
  (|CallParentFunction)
  (Variables|Default|SetmotorMeshInitialRot (Variables|/Script/Engine.SceneComponent|GetRelativeRotation (Variables|Default|GetMotorMesh))))

(event EventMoveForwardInputEvent
  (params (valueInput :type Float%20%28single-precision%29))
  (bind _returnvalue (== valueInput 0.0))
  (|CallParentFunction valueInput)
  (Utilities|IsValid (Variables|Default|GetplayerChar)
    (:Is%20Valid
      (bind _output_get (Variables|Default|SetmotorSplashAmount (Math|Interpolation|FInterpTo (Variables|Default|GetmotorSplashAmount) (Math|Float|SelectFloat (Math|Float|SelectFloat 1.5e+02 0.0 (!= (Variables|/Game/Assets/AmplifyAnimationPack/Blueprints/Character/BP_Character.BP_Character_C|GetInputRight (Variables|Default|GetplayerChar)) 0.0)) 4e+02 _returnvalue) (Utilities|Time|GetWorldDeltaSeconds) (Math|Float|SelectFloat 8.0 2.0 _returnvalue))))
      (Niagara|SetNiagaraVariable(Float) (Variables|Default|GetSplashParticleSystem) "SpawnRate" _output_get))))

(fn ConstructionScript
  (|CallParentFunction))