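; BP_SailBoatActor is a sailboat interactable whose driver mesh turns along with the player character's hand animation.
; BeginPlay stores the SailDriverMesh's initial rotation.
; Each tick, with a valid player, it reads the Boat_HandTurnAmount animation curve through the character's anim communicator and offsets the mesh's yaw from that initial value by the scaled result.
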(event EventBeginPlay
  (|CallParentFunction)
  (Variables|Default|SetdriverInitialRot (Variables|/Script/Engine.SceneComponent|GetRelativeRotation (Variables|Default|GetSailDriverMesh))))

(event EventTick
  (params (DeltaSeconds :type Float%20%28single-precision%29))
  (bind _playerchar (Variables|Default|GetplayerChar))
  (|CallParentFunction 0.0)
  (Utilities|IsValid _playerchar
    (:Is%20Valid
      (bind _asanim_instance (Utilities|Casting|CastToAnimInstance (Variables|/Game/Assets/AmplifyAnimationPack/Blueprints/Character/BP_Character.BP_Character_C|GetcharAnimCommunicator _playerchar)))
      (Transformation|SetRelativeRotation (Variables|Default|GetSailDriverMesh) (Math|Rotator|MakeRotator 0.0 0.0 (+ (.yaw (Variables|Default|GetdriverInitialRot)) (* (Animation|Curves|GetCurveValue _asanim_instance "Boat_HandTurnAmount") 23.0))) false false))))

(fn ConstructionScript
  (|CallParentFunction))