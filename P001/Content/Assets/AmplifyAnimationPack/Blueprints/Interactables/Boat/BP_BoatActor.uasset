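; Interactable boat actor that the player boards, switching the character to BP_BoatState and attaching it to the boat.
; Tick either bobs height, roll and pitch on a sine wave, or interpolates back toward the resting pose and triggers GetOutOfBoat at resting height.
; Enter and leave events toggle mesh physics and player collision volumes.
; While in boat state, look input rotates the boat's camera arm; movement and interact input forward to the character.
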(event Custom|CharacterEntered
  ;[1 1 1] Character entering/leaving boat events
  (Collision|SetCollisionEnabled (Variables|Default|GetPlayer_Detector) "NoCollision")
  (Collision|SetCollisionEnabled (Variables|Default|GetPlayer_Obstructor) "NoCollision")
  (Physics|SetSimulatePhysics (Variables|Default|GetMesh) true)
  (Variables|Default|SetisLerpingToOriginalPosRot true))

(event Custom|CharacterLeft
  ;[1 1 1] Character entering/leaving boat events
  (Collision|SetCollisionEnabled (Variables|Default|GetPlayer_Detector) "QueryOnly")
  (Collision|SetCollisionEnabled (Variables|Default|GetPlayer_Obstructor) "QueryAndPhysics")
  (Physics|SetSimulatePhysics (Variables|Default|GetMesh) false)
  (Variables|Default|SetisLerpingToOriginalPosRot false)
  (Variables|Default|SetplayerChar 0))

(event EventInputPossessEvent
  ;[1 1 1] Input Possession
  (Transformation|AttachActorToActor (Variables|Default|GetplayerChar) self "None" "KeepWorld" "KeepWorld" "KeepWorld" true)
  (Variables|Default|SetisLerpingToOriginalPosRot false))

(event EventTick
  (params (DeltaSeconds :type Float%20%28single-precision%29))
  ;[1 1 1] UE base events
  (if (Variables|Default|GetisLerpingToOriginalPosRot)
    (CallFunction|LerptoOriginalPosandRot)
    (else
      (CallFunction|WavePositionDisplacement))))

(event EventBeginPlay
  ;[1 1 1] UE base events
  (Variables|InitialValues|SetinitialPosZ (.z (Transformation|GetActorLocation)))
  (Variables|InitialValues|SetinitialRotator (Transformation|GetActorRotation)))

(event EventInteract
  (params (player :type BP%20Character%20Object%20Reference))
  ;[1 1 1] Interaction begin event
  (Default|ChangeCurrentState player "/Game/Assets/AmplifyAnimationPack/Blueprints/Character/CharacterStates/BP_BoatState.BP_BoatState_C")
  (Variables|Default|SetplayerChar player)
  (Default|UIHideInteractionUI player))

(event EventTurnInputEvent
  (params (valueInput :type Float%20%28single-precision%29))
  ;[1 1 1] Input Axis
  (Utilities|IsValid (Variables|Default|GetplayerChar)
    (:Is%20Valid
      (if (Utilities|CheckIsBoatState)
        (Transformation|AddRelativeRotation (Variables|Default|GetCameraArm) (Math|Rotator|MakeRotator 0.0 0.0 valueInput) false false)))))

(event EventMoveForwardInputEvent
  (params (valueInput :type Float%20%28single-precision%29))
  (bind _playerchar (Variables|Default|GetplayerChar))
  ;[1 1 1] Input Axis
  (Utilities|IsValid _playerchar
    (:Is%20Valid
      (if (Utilities|CheckIsBoatState)
        (Default|MoveForwardInputEvent _playerchar valueInput)))))

(event EventLookUpInputEvent
  (params (valueInput :type Float%20%28single-precision%29))
  (bind _playerchar (Variables|Default|GetplayerChar))
  (bind _cameraarm (Variables|Default|GetCameraArm))
  (bind _relativerotation (Variables|/Script/Engine.SceneComponent|GetRelativeRotation _cameraarm))
  ;[1 1 1] Input Axis
  (Utilities|IsValid _playerchar
    (:Is%20Valid
      (if (Utilities|CheckIsBoatState)
        (Transformation|SetRelativeRotation _cameraarm (Math|Rotator|MakeRotator 0.0 (Math|Float|Clamp(Float) (+ (.pitch _relativerotation) (* valueInput (select (Variables|/Game/Assets/AmplifyAnimationPack/Blueprints/Character/BP_Character.BP_Character_C|GetisYInverted _playerchar) -1.0 1.0))) -3e+01 3e+01) (.yaw _relativerotation)) false false)))))

(event EventMoveRightInputEvent
  (params (valueAxis :type Float%20%28single-precision%29))
  (bind _playerchar (Variables|Default|GetplayerChar))
  ;[1 1 1] Input Axis
  (Utilities|IsValid _playerchar
    (:Is%20Valid
      (if (Utilities|CheckIsBoatState)
        (Default|MoveRightInputEvent _playerchar valueAxis)))))

(event EventInteractInputEvent
  (bind _playerchar (Variables|Default|GetplayerChar))
  ;[1 1 1] Input Actions
  (Utilities|IsValid _playerchar
    (:Is%20Valid
      (if (Utilities|CheckIsBoatState)
        (Default|InteractInputEvent _playerchar)))))

(fn ConstructionScript)

(fn WavePositionDisplacement
  (bind _returnvalue (Transformation|GetActorLocation))
  (bind _output_get (Variables|WaveSystem|SetwaveTimer (+ (Variables|WaveSystem|GetwaveTimer) (Utilities|Time|GetWorldDeltaSeconds))))
  (Transformation|SetActorLocation (Math|Vector|MakeVector (.x _returnvalue) (.y _returnvalue) (+ (Variables|InitialValues|GetinitialPosZ) (* (Variables|WaveSystem|GetbuyoancyHeightAmount) (Math|Trig|Sin(Radians) _output_get)))) false false)
  (Transformation|SetActorRotation (Math|Rotator|MakeRotator (.roll (Math|Rotator|CombineRotators (Variables|InitialValues|GetinitialRotator) (Math|Rotator|MakeRotator (* (Math|Trig|Sin(Radians) _output_get) (Variables|WaveSystem|GetbuyoancyRollAmount)) (* (Math|Trig|Sin(Radians) _output_get) (Variables|WaveSystem|GetbuyoancyPitchAmount)) 0.0))) (.pitch (Math|Rotator|CombineRotators (Variables|InitialValues|GetinitialRotator) (Math|Rotator|MakeRotator (* (Math|Trig|Sin(Radians) _output_get) (Variables|WaveSystem|GetbuyoancyRollAmount)) (* (Math|Trig|Sin(Radians) _output_get) (Variables|WaveSystem|GetbuyoancyPitchAmount)) 0.0))) (.yaw (Transformation|GetActorRotation)))))

(fn LerptoOriginalPosandRot
  (bind _returnvalue (Utilities|Time|GetWorldDeltaSeconds))
  (bind _returnvalue_2 (Transformation|GetActorRotation))
  (bind _returnvalue_3 (Transformation|GetActorLocation))
  (Transformation|SetActorLocation (Math|Vector|MakeVector (.x _returnvalue_3) (.y _returnvalue_3) (Math|Interpolation|FInterptoConstant (.z _returnvalue_3) (Variables|InitialValues|GetinitialPosZ) _returnvalue 45.0)) false false)
  (Transformation|SetActorRotation (Math|Interpolation|RInterpTo _returnvalue_2 (Math|Rotator|MakeRotator 0.0 0.0 (.Yaw (Math|Rotator|BreakRotator _returnvalue_2))) _returnvalue 7e+01))
  (Variables|WaveSystem|SetwaveTimer 0.0)
  (if (< (Math|Float|Absolute(Float) (- (.z (Transformation|GetActorLocation)) (Variables|InitialValues|GetinitialPosZ))) 0.001)
    (CallFunction|TriggerCharGettingOut)))

(fn PrepareforCharGettingOut
  (Physics|SetPhysicsLinearVelocity (Variables|Default|GetMesh) "0, 0, 0" false "None")
  (Variables|Default|SetisLerpingToOriginalPosRot true))

(fn TriggerCharGettingOut
  (bind _playerchar (Variables|Default|GetplayerChar))
  (Utilities|IsValid _playerchar
    (:Is%20Valid
      (bind _asbp_boat_state (Utilities|Casting|CastToBP_BoatState (Variables|/Game/Assets/AmplifyAnimationPack/Blueprints/Character/BP_Character.BP_Character_C|GetcurrentState _playerchar)))
      (Default|GetOutOfBoat _asbp_boat_state))))

(fn CheckResetPlayerCrouch
  (return false))