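; Wall lever interactable that shows a push prompt and registers itself as the overlapping BP_Character's interaction target.
; Interact puts the player in BP_InteractionState, aligns them to the PlayerPosition point and lever-relative facing, then picks the character's interaction animation type from IsClosed.
; Open and Close, not called within this Blueprint, play the handle's down and up animations and set IsClosed, with Open setting it true.
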(event OnComponentBeginOverlap(Player_Detector)
  (params (OverlappedComponent :type Primitive%20Component%20Object%20Reference) (OtherActor :type Actor%20Object%20Reference) (OtherComp :type Primitive%20Component%20Object%20Reference) (OtherBodyIndex :type Integer) (bFromSweep :type Boolean) (SweepResult :type Hit%20Result%20Structure%20%28by%20ref%29))
  ;[1 1 1] Player Detection
  (bind _asbp_character (Utilities|Casting|CastToBP_Character OtherActor))
  (Variables|/Game/Assets/AmplifyAnimationPack/Blueprints/Character/BP_Character.BP_Character_C|SetobjectToInteract _asbp_character self)
  (Default|UIShowInteractionUI _asbp_character "Press E to Push lever"))

(event OnComponentEndOverlap(Player_Detector)
  (params (OverlappedComponent :type Primitive%20Component%20Object%20Reference) (OtherActor :type Actor%20Object%20Reference) (OtherComp :type Primitive%20Component%20Object%20Reference) (OtherBodyIndex :type Integer))
  ;[1 1 1] Player Detection
  (bind _asbp_character (Utilities|Casting|CastToBP_Character OtherActor))
  (Variables|/Game/Assets/AmplifyAnimationPack/Blueprints/Character/BP_Character.BP_Character_C|SetobjectToInteract _asbp_character 0)
  (Default|UIHideInteractionUI _asbp_character))

(event EventBeginPlay
  (Variables|Default|SetisClosed false))

(event EventInteract
  (params (player :type BP%20Character%20Object%20Reference))
  (bind _returnvalue (Transformation|GetActorRotation))
  (bind _returnvalue_2 (Transformation|GetActorLocation player))
  (bind _playerposition (Variables|Default|GetPlayerPosition))
  (bind _returnvalue_3 (Transformation|GetWorldLocation _playerposition))
  (Default|ChangeCurrentState player "/Game/Assets/AmplifyAnimationPack/Blueprints/Character/CharacterStates/BP_InteractionState.BP_InteractionState_C")
  (Default|AdjustPosition player _returnvalue_2 (- (Math|Vector|MakeVector (.x _returnvalue_3) (.y _returnvalue_3) (.z (Transformation|GetActorLocation player))) _returnvalue_2) false false true)
  (Default|AdjustRotation player (Math|Rotator|GetRotationXVector (Math|Rotator|MakeRotator (.roll _returnvalue) (.pitch _returnvalue) (+ (.yaw _returnvalue) 9e+01))) true 7.0)
  (Default|SetInteractionTypeVal (Variables|/Game/Assets/AmplifyAnimationPack/Blueprints/Character/BP_Character.BP_Character_C|GetcharAnimCommunicator player) (select (Variables|Default|GetisClosed) "NewEnumerator4" "NewEnumerator3")))

(fn ConstructionScript)

(fn Open
  (Components|Animation|PlayAnimation (Variables|Default|GetHandle) "/Game/Assets/AmplifyAnimationPack/Animations/Interactables/WallLever_Down_Anim.WallLever_Down_Anim" false)
  (Variables|Default|SetisClosed true))

(fn Close
  (Components|Animation|PlayAnimation (Variables|Default|GetHandle) "/Game/Assets/AmplifyAnimationPack/Animations/Interactables/WallLever_Up_Anim.WallLever_Up_Anim" false)
  (Variables|Default|SetisClosed false))

(fn CheckResetPlayerCrouch
  (return true))