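; BP_BowActor is a bow weapon that fires arrow projectiles for its owner.
; The construction script snaps a display Arrow to the mesh's stringSocket, shown on attach or aim and hidden on detach or fire.
; Firing spawns BP_BowProjectile at that arrow, aimed at a point ahead of the owner's camera.
; Aim and shoot events play bow animations whose asset names are reversed: aim plays Release, shoot plays Aim.
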(event Custom|AimArrow
  ;[1 1 1] Bow specific events
  (Components|Animation|PlayAnimation (Variables|Character|GetMesh) "/Game/Assets/AmplifyAnimationPack/Animations/Weapons/Bow_Release_Anim.Bow_Release_Anim" false)
  (Rendering|SetVisibility (Variables|Default|GetArrow) true false))

(event Custom|ShootArrow
  ;[1 1 1] Bow specific events
  (Components|Animation|PlayAnimation (Variables|Character|GetMesh) "/Game/Assets/AmplifyAnimationPack/Animations/Weapons/Bow_Aim_Anim.Bow_Aim_Anim" false))

(event EventWeaponFire
  (params (weaponOwner :type BP%20Character%20Object%20Reference))
  (bind _arrow (Variables|Default|GetArrow))
  (bind _camera (Variables|/Game/Assets/AmplifyAnimationPack/Blueprints/Character/BP_Character.BP_Character_C|GetCamera weaponOwner))
  (Rendering|SetVisibility _arrow false false)
  (bind _returnvalue (Game|SpawnActorfromClass "/Game/Assets/AmplifyAnimationPack/Blueprints/Weapons/BP_BowProjectile.BP_BowProjectile_C" (Transformation|GetWorldTransform _arrow) "Undefined" 0 0))
  (Default|FireArrow _returnvalue (Math|Vector|GetForwardVector (Math|Rotator|FindLookatRotation (Transformation|GetWorldLocation _arrow) (+ (Transformation|GetWorldLocation _camera) (* (Math|Vector|GetForwardVector _camera) 5e+02))))))

(event EventWeaponAttachedEvent
  (|CallParentFunction)
  (Rendering|SetVisibility (Variables|Default|GetArrow) true false))

(event EventWeaponUnattachedEvent
  (|CallParentFunction)
  (Rendering|SetVisibility (Variables|Default|GetArrow) false false))

(fn ConstructionScript
  (|CallParentFunction)
  (Transformation|AttachComponentToComponent (Variables|Default|GetArrow) (Variables|Character|GetMesh) "stringSocket" "SnapToTarget" "SnapToTarget" "KeepWorld" false))