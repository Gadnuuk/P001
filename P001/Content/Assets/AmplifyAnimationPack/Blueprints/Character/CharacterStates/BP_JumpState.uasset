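; Character state for jumping: sets jump velocity, heavier gravity, capsule radius and sprint-dependent speed and camera distance, restoring most on exit.
; Each update pushes movement along the entry direction if the character was moving, while traces detect landing, switch to swim or hang states, or time the fall.
; Obstacle actors block landing and can re-enter the state for a second jump.
; Input and vertical velocity feed the animation communicator.
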(fn EnterState
  (params (prevStateClass :type BP%20Character%20State%20Base%20Class%20Reference))
  (bind _charref (Variables|Default|GetcharRef))
  (bind _charref_2 (Variables|Default|GetcharRef))
  (bind _charref_3 (Variables|Default|GetcharRef))
  (bind _charactermovement (Variables|/Script/Engine.Character|GetCharacterMovement _charref_2))
  (bind _charanimcommunicator (Variables|/Game/Assets/AmplifyAnimationPack/Blueprints/Character/BP_Character.BP_Character_C|GetcharAnimCommunicator _charref_2))
  (|CallParentFunction 0)
  (bind _curentvalue (Default|GetMovementStateVal (Variables|/Game/Assets/AmplifyAnimationPack/Blueprints/Character/BP_Character.BP_Character_C|GetcharAnimCommunicator _charref)))
  (Default|SetNewCapsuleRadius _charref 23.0 0.0)
  (Variables|/Script/Engine.CharacterMovementComponent|SetMaxWalkSpeed (Variables|/Script/Engine.Character|GetCharacterMovement _charref) (Math|Float|SelectFloat 7.5e+02 5.5e+02 (Utilities|Enum|Equal(Enum) _curentvalue "NewEnumerator1")))
  (Variables|/Game/Assets/AmplifyAnimationPack/Blueprints/Character/BP_Character.BP_Character_C|SetcameraDistanceTarget _charref_3 (Math|Float|SelectFloat (Variables|/Game/Assets/AmplifyAnimationPack/Blueprints/Character/BP_Character.BP_Character_C|GetcameraDistanceSprint _charref_3) (Variables|/Game/Assets/AmplifyAnimationPack/Blueprints/Character/BP_Character.BP_Character_C|GetcameraDistanceDefault _charref_3) (Utilities|Enum|Equal(Enum) _curentvalue "NewEnumerator1")))
  (Default|SetCanLandVal _charanimcommunicator false)
  (Default|SetJumpTimertoFallVal _charanimcommunicator 0.0)
  (Default|SetMovementStateVal _charanimcommunicator "NewEnumerator3")
  (Variables|Default|SetentryDirection (Transformation|GetActorForwardVector _charref_2))
  (Variables|/Script/Engine.CharacterMovementComponent|SetJumpZVelocity _charactermovement (Variables|/Game/Assets/AmplifyAnimationPack/Blueprints/Character/BP_Character.BP_Character_C|GetjumpVelocity _charref_2))
  (Variables|/Script/Engine.CharacterMovementComponent|SetGravityScale _charactermovement 2.267)
  (Variables|Default|SetisJumpForward (> (Math|Vector|VectorLength (Transformation|GetVelocity _charref_2)) 0.0)))

(fn UpdateState
  (params (deltaTime :type Float%20%28single-precision%29))
  (bind _charref (Variables|Default|GetcharRef))
  (bind _charref_2 (Variables|Default|GetcharRef))
  (bind _charref_3 (Variables|Default|GetcharRef))
  (bind _charref_4 (Variables|Default|GetcharRef))
  (bind _charanimcommunicator (Variables|/Game/Assets/AmplifyAnimationPack/Blueprints/Character/BP_Character.BP_Character_C|GetcharAnimCommunicator _charref_4))
  (bind _charanimcommunicator_2 (Variables|/Game/Assets/AmplifyAnimationPack/Blueprints/Character/BP_Character.BP_Character_C|GetcharAnimCommunicator _charref_3))
  (|CallParentFunction 0.0)
  (bind _curentvalue (Default|GetMovementStateVal (Variables|/Game/Assets/AmplifyAnimationPack/Blueprints/Character/BP_Character.BP_Character_C|GetcharAnimCommunicator (Variables|Default|GetcharRef))))
  (Pawn|Input|AddMovementInput _charref (Variables|Default|GetentryDirection) (Math|Float|SelectFloat 1.0 0.0 (and (Utilities|Enum|Equal(Enum) _curentvalue "NewEnumerator3") (Variables|Default|GetisJumpForward))) true)
  (bind (_canland _hitresult) (Default|JumpLinetraceDetector _charref))
  (if (and (> (.z (.ImpactNormal (Collision|BreakHitResult _hitresult))) 0.75) _canland)
    (if (Utilities|Enum|Equal(Enum) (Collision|GetCollisionObjectType (.HitComponent (Collision|BreakHitResult _hitresult))) "ECC_GameTraceChannel5")
      (Default|ChangeCurrentState _charref_2 "/Game/Assets/AmplifyAnimationPack/Blueprints/Character/CharacterStates/BP_SwimState.BP_SwimState_C")
      (else
        (Default|SetCanLandVal _charanimcommunicator (not (== (Utilities|GetClass (.HitActor (Collision|BreakHitResult _hitresult))) "/Game/Assets/AmplifyAnimationPack/Blueprints/Interactables/BP_ObstacleActor.BP_ObstacleActor_C")))
        (bind (_groundhitresult _isgrounded) (Default|GroundSpheretraceDetector _charref_2))
        (if (Math|Boolean|ANDBoolean (== (Utilities|GetClass (.HitActor (Collision|BreakHitResult _groundhitresult))) "/Game/Assets/AmplifyAnimationPack/Blueprints/Interactables/BP_ObstacleActor.BP_ObstacleActor_C") (> (.z (.ImpactNormal (Collision|BreakHitResult _groundhitresult))) 0.9) _isgrounded (== (Variables|Default|GetjumpsMade) 1))
          (CallFunction|EnterState)
          (Default|SetJumpWillSecondJumpVal _charanimcommunicator_2 true)
          (Variables|/Script/Engine.CharacterMovementComponent|SetJumpZVelocity (Variables|/Script/Engine.Character|GetCharacterMovement _charref_3) (Variables|/Game/Assets/AmplifyAnimationPack/Blueprints/Character/BP_Character.BP_Character_C|GetjumpVelocity_Second _charref_3))
          (Variables|Default|SetisJumpForward true)
          (else
            (Default|SetJumpWillSecondJumpVal _charanimcommunicator_2 false)))))
    (else
      (bind _curentvalue_2 (Default|GetJumpTimertoFallVal _charanimcommunicator))
      (Default|SetJumpTimertoFallVal _charanimcommunicator (+ _curentvalue_2 deltaTime))
      (bind _ishitting (Default|ClimbLinetraceHangStart _charref_4))
      (if _ishitting
        (Default|ChangeCurrentState (Variables|Default|GetcharRef) "/Game/Assets/AmplifyAnimationPack/Blueprints/Character/CharacterStates/BP_HangState.BP_HangState_C")))))

(fn UpdateStateAnimation
  (bind _charref (Variables|Default|GetcharRef))
  (bind _charanimcommunicator (Variables|/Game/Assets/AmplifyAnimationPack/Blueprints/Character/BP_Character.BP_Character_C|GetcharAnimCommunicator _charref))
  (|CallParentFunction)
  (CallFunction|SetCharVelocityAnim)
  (bind _curentvalue (Default|GetMovementStateVal (Variables|/Game/Assets/AmplifyAnimationPack/Blueprints/Character/BP_Character.BP_Character_C|GetcharAnimCommunicator (Variables|Default|GetcharRef))))
  (if (Utilities|Enum|Equal(Enum) _curentvalue "NewEnumerator3")
    (bind _curentvalue_2 (Default|GetInputRightVal _charanimcommunicator))
    (bind _curentvalue_3 (Default|GetInputFwdVal _charanimcommunicator))
    (Default|SetSpeedVal _charanimcommunicator (Math|Float|Clamp(Float) (+ (Math|Float|Absolute(Float) _curentvalue_2) (Math|Float|Absolute(Float) _curentvalue_3))))
    (else
      (return))))

(fn InputMoveForward
  (params (inputVal :type Float%20%28single-precision%29))
  (bind _charref (Variables|Default|GetcharRef))
  (|CallParentFunction 0.0)
  (bind _output_get (Variables|/Game/Assets/AmplifyAnimationPack/Blueprints/Character/BP_Character.BP_Character_C|SetInputForward _charref inputVal))
  (Default|SetInputFwdVal (Variables|/Game/Assets/AmplifyAnimationPack/Blueprints/Character/BP_Character.BP_Character_C|GetcharAnimCommunicator _charref) _output_get))

(fn InputMoveRight
  (params (inputVal :type Float%20%28single-precision%29))
  (bind _charref (Variables|Default|GetcharRef))
  (|CallParentFunction 0.0)
  (bind _output_get (Variables|/Game/Assets/AmplifyAnimationPack/Blueprints/Character/BP_Character.BP_Character_C|SetInputRight _charref inputVal))
  (Default|SetInputRightVal (Variables|/Game/Assets/AmplifyAnimationPack/Blueprints/Character/BP_Character.BP_Character_C|GetcharAnimCommunicator _charref) _output_get))

(fn ExitState
  (bind _charref (Variables|Default|GetcharRef))
  (bind _charref_2 (Variables|Default|GetcharRef))
  (bind _charactermovement (Variables|/Script/Engine.Character|GetCharacterMovement _charref))
  (|CallParentFunction)
  (Variables|Default|SetjumpsMade 0)
  (Variables|/Script/Engine.CharacterMovementComponent|SetGravityScale _charactermovement 1.0)
  (Variables|/Script/Engine.CharacterMovementComponent|SetMaxWalkSpeed _charactermovement 5.5e+02)
  (Variables|/Game/Assets/AmplifyAnimationPack/Blueprints/Character/BP_Character.BP_Character_C|SetcameraDistanceTarget _charref_2 (Variables|/Game/Assets/AmplifyAnimationPack/Blueprints/Character/BP_Character.BP_Character_C|GetcameraDistanceDefault _charref_2)))

(fn SetCharVelocityAnim
  (bind _charref (Variables|Default|GetcharRef))
  (Default|SetCharVelocityVal (Variables|/Game/Assets/AmplifyAnimationPack/Blueprints/Character/BP_Character.BP_Character_C|GetcharAnimCommunicator _charref) (.z (Transformation|GetVelocity _charref))))