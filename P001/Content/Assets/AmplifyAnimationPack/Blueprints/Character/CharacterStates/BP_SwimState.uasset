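; Character state for swimming in the Amplify Animation Pack, covering water entry, surface and underwater movement, and climbing out.
; Entry picks a fall-impact or dive-jump action, which gives way to Swim once traces or velocity allow.
; Movement follows control rotation, partly scaled by the Swim_MovementAmount animation curve, with surface detection limiting vertical motion and adjusting braking.
; Jump climbs unobstructed ledges, holding it ascends underwater, and ground detection switches to the grounded state.
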(fn EnterState
  (params (prevStateClass :type BP%20Character%20State%20Base%20Class%20Reference))
  (bind _returnvalue (== prevStateClass "/Game/Assets/AmplifyAnimationPack/Blueprints/Character/CharacterStates/BP_BoatState.BP_BoatState_C"))
  (bind _charref (Variables|Default|GetcharRef))
  (bind _charanimcommunicator (Variables|/Game/Assets/AmplifyAnimationPack/Blueprints/Character/BP_Character.BP_Character_C|GetcharAnimCommunicator _charref))
  (bind _charactermovement (Variables|/Script/Engine.Character|GetCharacterMovement _charref))
  (bind _returnvalue_2 (AI|Components|NavMovement|IsFalling _charactermovement))
  (bind _returnvalue_3 (or _returnvalue_2 _returnvalue))
  (|CallParentFunction 0)
  (Collision|SetCollisionEnabled (Variables|/Script/Engine.Character|GetCapsuleComponent _charref) "QueryAndPhysics")
  (Variables|Default|SetcanMove false)
  (if _returnvalue_3
    (Variables|/Script/Engine.CharacterMovementComponent|SetBrakingDecelerationSwimming _charactermovement (Math|Float|SelectFloat 6e+03 7e+02 (< (.z (Transformation|GetVelocity _charref)) -9e+02))))
  (Default|SetSwimActionVal _charanimcommunicator (select _returnvalue_3 "NewEnumerator13" "NewEnumerator10"))
  (Pawn|Components|CharacterMovement|SetMovementMode _charactermovement (select _returnvalue_3 "MOVE_Swimming" "MOVE_Flying") 0)
  (Default|SetMovementStateVal _charanimcommunicator "NewEnumerator26")
  (Default|SetSpeedVal _charanimcommunicator 0.0))

(fn UpdateStateAnimation
  (bind _charref (Variables|Default|GetcharRef))
  (bind _charref_2 (Variables|Default|GetcharRef))
  (bind _charref_3 (Variables|Default|GetcharRef))
  (bind _charref_4 (Variables|Default|GetcharRef))
  (bind _returnvalue (Transformation|GetVelocity _charref_4))
  (bind _charanimcommunicator (Variables|/Game/Assets/AmplifyAnimationPack/Blueprints/Character/BP_Character.BP_Character_C|GetcharAnimCommunicator _charref_4))
  (bind _charanimcommunicator_2 (Variables|/Game/Assets/AmplifyAnimationPack/Blueprints/Character/BP_Character.BP_Character_C|GetcharAnimCommunicator _charref))
  (bind _charanimcommunicator_3 (Variables|/Game/Assets/AmplifyAnimationPack/Blueprints/Character/BP_Character.BP_Character_C|GetcharAnimCommunicator _charref_3))
  (bind _charanimcommunicator_4 (Variables|/Game/Assets/AmplifyAnimationPack/Blueprints/Character/BP_Character.BP_Character_C|GetcharAnimCommunicator _charref_2))
  (|CallParentFunction)
  (bind _curentvalue (Default|GetSwimActionVal (Variables|/Game/Assets/AmplifyAnimationPack/Blueprints/Character/BP_Character.BP_Character_C|GetcharAnimCommunicator (Variables|Default|GetcharRef))))
  (switch Utilities|FlowControl|Switch|SwitchonCharacter_SwimActions_Enum _curentvalue
    (:NewEnumerator11
      (bind _hashit (Default|SwimLinetraceDiveEnd _charref_4))
      (if _hashit
        (Default|SetSwimActionVal (Variables|/Game/Assets/AmplifyAnimationPack/Blueprints/Character/BP_Character.BP_Character_C|GetcharAnimCommunicator (Variables|Default|GetcharRef)) "NewEnumerator12")
        (Variables|/Script/Engine.CharacterMovementComponent|SetBrakingDecelerationSwimming (Variables|/Script/Engine.Character|GetCharacterMovement (Variables|Default|GetcharRef)) 5e+01 :!label _label)
        (Variables|Default|SetcanMove true)
        (Default|SetNewCapsuleRadius (Variables|Default|GetcharRef) 7e+01 0.0)))
    (:NewEnumerator13
      (CallFunction|DetectSurface)
      (Default|SetCharVelocityVal _charanimcommunicator (.z _returnvalue))
      (bind _curentvalue_2 (Default|GetSwimIsSurfaceVal _charanimcommunicator))
      (if (or (and (>= (.z _returnvalue) -7e+01) (not _curentvalue_2)) (>= (.z _returnvalue) -15.0))
        (Default|SetSwimActionVal _charanimcommunicator_2 "NewEnumerator12")
        (goto _label)))
    (:NewEnumerator12
      (bind _curentvalue_3 (Default|GetInputRightVal _charanimcommunicator_3))
      (bind _curentvalue_4 (Default|GetInputFwdVal _charanimcommunicator_3))
      (bind _currentvalue (Default|SetSpeedVal _charanimcommunicator_2 (Math|Float|Clamp(Float) (+ (Math|Float|Absolute(Float) _curentvalue_4) (Math|Float|Absolute(Float) _curentvalue_3) (Math|Float|Absolute(Float) (Variables|Default|GetinputJumpHold))))))
      (Default|SetSwimDirZVal _charanimcommunicator_2 (.z (Transformation|GetVelocity (Variables|Default|GetcharRef))))
      (CallFunction|DetectSurface)
      (CallFunction|SetDirection)
      (if (== _currentvalue 0.0)
        (bind _curentvalue_5 (Default|GetFramestoStopMovingVal _charanimcommunicator_4))
        (Default|SetFramestoStopMovVal _charanimcommunicator_4 (+ _curentvalue_5 1))
        (else
          (Default|SetFramestoStopMovVal _charanimcommunicator_4))))))

(fn InputMoveForward
  (params (inputVal :type Float%20%28single-precision%29))
  (bind _charref (Variables|Default|GetcharRef))
  (bind _returnvalue (Pawn|GetControlRotation _charref :!class /Script/Engine.Pawn))
  (bind _charanimcommunicator (Variables|/Game/Assets/AmplifyAnimationPack/Blueprints/Character/BP_Character.BP_Character_C|GetcharAnimCommunicator _charref))
  (bind _returnvalue_2 (Math|Vector|GetForwardVector _returnvalue))
  (|CallParentFunction 0.0)
  (bind _output_get (Variables|/Game/Assets/AmplifyAnimationPack/Blueprints/Character/BP_Character.BP_Character_C|SetInputForward _charref (Math|Interpolation|FInterpTo (Variables|/Game/Assets/AmplifyAnimationPack/Blueprints/Character/BP_Character.BP_Character_C|GetInputForward _charref) inputVal 0.05 2e+01)))
  (bind _asanim_instance (Utilities|Casting|CastToAnimInstance _charanimcommunicator))
  (bind _currentval (Default|SetInputFwdVal _charanimcommunicator _output_get))
  (bind _curentvalue (Default|GetSwimIsSurfaceVal _charanimcommunicator))
  (Pawn|Input|AddMovementInput (Variables|Default|GetcharRef) (Math|Vector|MakeVector (.x _returnvalue_2) (.y _returnvalue_2) (Math|Float|SelectFloat (Math|Float|SelectFloat (.z _returnvalue_2) 0.0 (< (.z _returnvalue_2) -0.5)) (.z _returnvalue_2) _curentvalue)) (Math|Float|SelectFloat (Math|Float|SelectFloat (Math|Float|SelectFloat _currentval (* (Animation|Curves|GetCurveValue _asanim_instance "Swim_MovementAmount") (Math|Float|Sign(Float) _currentval)) _curentvalue) 0.0 (!= _currentval 0.0)) 0.0 (Variables|Default|GetcanMove)) false))

(fn InputMoveRight
  (params (inputVal :type Float%20%28single-precision%29))
  (bind _charref (Variables|Default|GetcharRef))
  (bind _returnvalue (Pawn|GetControlRotation _charref :!class /Script/Engine.Pawn))
  (bind _charanimcommunicator (Variables|/Game/Assets/AmplifyAnimationPack/Blueprints/Character/BP_Character.BP_Character_C|GetcharAnimCommunicator _charref))
  (bind _returnvalue_2 (Math|Vector|GetRightVector _returnvalue))
  (bind _output_get (Variables|/Game/Assets/AmplifyAnimationPack/Blueprints/Character/BP_Character.BP_Character_C|SetInputRight _charref (Math|Interpolation|FInterpTo (Variables|/Game/Assets/AmplifyAnimationPack/Blueprints/Character/BP_Character.BP_Character_C|GetInputRight _charref) inputVal 0.05 2e+01)))
  (bind _asanim_instance (Utilities|Casting|CastToAnimInstance _charanimcommunicator))
  (bind _currentval (Default|SetInputRightVal _charanimcommunicator _output_get))
  (bind _curentvalue (Default|GetSwimIsSurfaceVal _charanimcommunicator))
  (Pawn|Input|AddMovementInput (Variables|Default|GetcharRef) (Math|Vector|MakeVector (.x _returnvalue_2) (.y _returnvalue_2) (Math|Float|SelectFloat (Math|Float|SelectFloat 0.0 (Math|Float|Max(Float) (.z _returnvalue_2) 0.0) (< (.z _returnvalue_2) -0.5)) (.z _returnvalue_2) _curentvalue)) (Math|Float|SelectFloat (Math|Float|SelectFloat (Math|Float|SelectFloat _currentval (* (Animation|Curves|GetCurveValue _asanim_instance "Swim_MovementAmount") (Math|Float|Sign(Float) _currentval)) _curentvalue) 0.0 (!= _currentval 0.0)) 0.0 (Variables|Default|GetcanMove)) false))

(fn InputJump
  (bind _charref (Variables|Default|GetcharRef))
  (bind _charref_2 (Variables|Default|GetcharRef))
  (bind _charref_3 (Variables|Default|GetcharRef))
  (bind _charref_4 (Variables|Default|GetCharRef))
  (bind _charref_5 (Variables|Default|GetcharRef))
  (bind _returnvalue (Transformation|GetActorForwardVector _charref_4))
  (bind _returnvalue_2 (Transformation|GetActorLocation _charref_4))
  (bind _charanimcommunicator (Variables|/Game/Assets/AmplifyAnimationPack/Blueprints/Character/BP_Character.BP_Character_C|GetcharAnimCommunicator _charref_5))
  (bind _returnvalue_3 (* _returnvalue 3e+01))
  (bind (_x _y _z) (Math|Vector|BreakVector _returnvalue_2))
  (bind _returnvalue_4 (+ _returnvalue_2 _returnvalue_3))
  (|CallParentFunction)
  (bind _curentvalue (Default|GetSwimActionVal (Variables|/Game/Assets/AmplifyAnimationPack/Blueprints/Character/BP_Character.BP_Character_C|GetcharAnimCommunicator _charref)))
  (if (Utilities|Enum|Equal(Enum) _curentvalue "NewEnumerator12")
    (bind (_hashit _impactnormal) (Default|SwimLinetraceClimb _charref))
    (if _hashit
      (bind _hashit_2 (Default|SwimLinetraceClimbDetectObstacle _charref_2))
      (if _hashit_2
        (return)
        (else
          (Pawn|Components|CharacterMovement|SetMovementMode (Variables|/Script/Engine.Character|GetCharacterMovement _charref_2) "MOVE_Flying" 0)
          (Default|SetSwimActionVal _charanimcommunicator "NewEnumerator14")
          (Default|SetMovementStateVal _charanimcommunicator "NewEnumerator0")
          (Default|SetSpeedVal _charanimcommunicator 0.0)
          (Default|AdjustRotation _charref_4 (* _impactnormal -1.0) false 0.0)
          (bind _impactpoint (Default|SwimLinetraceClimbHeight _charref_4))
          (Default|AdjustPosition _charref_3 _returnvalue_2 (Math|Vector|MakeVector (- (.x _returnvalue_4) _x) (- (.y _returnvalue_4) _y) (- (- (.z _impactpoint) _z) 54.5)) false true false)
          (Default|SetNewCapsuleRadius _charref_3 0.0 0.0)
          (Components|Capsule|SetCapsuleHalfHeight (Variables|/Script/Engine.Character|GetCapsuleComponent _charref_3) 0.0 true)
          (Variables|Default|SetcanMove false))))))

(fn DetectSurface
  (bind _charref (Variables|Default|GetcharRef))
  (bind _hashit (Default|SwimLinetraceSurface _charref))
  (Default|SetSwimIsSurfaceVal (Variables|/Game/Assets/AmplifyAnimationPack/Blueprints/Character/BP_Character.BP_Character_C|GetcharAnimCommunicator _charref) (not _hashit)))

(fn SetDirection
  (bind _charref (Variables|Default|GetcharRef))
  (bind _charanimcommunicator (Variables|/Game/Assets/AmplifyAnimationPack/Blueprints/Character/BP_Character.BP_Character_C|GetcharAnimCommunicator _charref))
  (bind _newdirection (Default|UpdateDirection _charref false))
  (bind _curentvalue (Default|GetSpeedVal _charanimcommunicator))
  (if (> _curentvalue 0.0)
    (Default|SetDirectionVal _charanimcommunicator _newdirection)
    (else
      (return))))

(fn UpdateState
  (params (deltaTime :type Float%20%28single-precision%29))
  (bind _charref (Variables|Default|GetcharRef))
  (bind _charref_2 (Variables|Default|GetcharRef))
  (bind _returnvalue (Transformation|GetVelocity _charref))
  (bind _charanimcommunicator (Variables|/Game/Assets/AmplifyAnimationPack/Blueprints/Character/BP_Character.BP_Character_C|GetcharAnimCommunicator _charref))
  (bind _returnvalue_2 (Math|Vector|VectorLength _returnvalue))
  (|CallParentFunction 0.0)
  (bind _curentvalue (Default|GetSwimActionVal _charanimcommunicator))
  (bind _curentvalue_2 (Default|GetSwimIsSurfaceVal _charanimcommunicator))
  (CallFunction|UpdateRotation _returnvalue_2)
  (Default|BoatLinetrace _charref_2 1.5e+02)
  (if (and (!= _returnvalue_2 0.0) (Utilities|Enum|Equal(Enum) _curentvalue "NewEnumerator12"))
    (Variables|/Script/Engine.CharacterMovementComponent|SetBrakingDecelerationSwimming (Variables|/Script/Engine.Character|GetCharacterMovement _charref_2) (Math|Float|SelectFloat 1.4e+03 2e+01 _curentvalue_2))
    (CallFunction|GroundDetection)))

(fn InputJumpHold
  (params (inputVal :type Float%20%28single-precision%29))
  (bind _charref (Variables|Default|GetcharRef))
  (bind _charanimcommunicator (Variables|/Game/Assets/AmplifyAnimationPack/Blueprints/Character/BP_Character.BP_Character_C|GetcharAnimCommunicator _charref))
  (|CallParentFunction 0.0)
  (bind _asanim_instance (Utilities|Casting|CastToAnimInstance _charanimcommunicator))
  (bind _curentvalue (Default|GetSwimIsSurfaceVal _charanimcommunicator))
  (bind _hashit (Default|SwimLinetraceIsHeadingtoSurface (Variables|Default|GetcharRef)))
  (bind _output_get (Variables|Default|SetinputJumpHold (Math|Float|SelectFloat (Math|Interpolation|FInterpTo (Variables|Default|GetinputJumpHold) inputVal 0.05 2e+01) 0.0 (Math|Boolean|ANDBoolean (not _curentvalue) (Variables|Default|GetcanMove) _hashit))))
  (Pawn|Input|AddMovementInput (Variables|Default|GetcharRef) (Math|Vector|MakeVector 0.0 0.0 1.0) (Math|Float|SelectFloat (Math|Float|SelectFloat (* (Animation|Curves|GetCurveValue _asanim_instance "Swim_MovementAmount") (Math|Float|Sign(Float) _output_get)) 0.0 (!= _output_get 0.0)) 0.0 (Math|Boolean|ANDBoolean (not _curentvalue) (Variables|Default|GetcanMove) _hashit)) false))

(fn UpdateRotation
  (params (currentVelocity :type Float%20%28single-precision%29))
  (bind _charref (Variables|Default|GetcharRef))
  (Variables|/Game/Assets/AmplifyAnimationPack/Blueprints/Character/BP_Character.BP_Character_C|SetcurrentRotationRate _charref (Math|Float|SelectFloat (Variables|/Game/Assets/AmplifyAnimationPack/Blueprints/Character/BP_Character.BP_Character_C|GetswimRotationRate _charref) (Variables|/Game/Assets/AmplifyAnimationPack/Blueprints/Character/BP_Character.BP_Character_C|GetswimAccelRotationRate _charref) (> currentVelocity 2e+02)))
  (Default|RotateCharacter _charref (Variables|Default|GetcanMove) false))

(fn InputInteract
  (bind _charref (Variables|Default|GetcharRef))
  (bind _objecttointeract (Variables|/Game/Assets/AmplifyAnimationPack/Blueprints/Character/BP_Character.BP_Character_C|GetobjectToInteract _charref))
  (|CallParentFunction)
  (Utilities|IsValid (Utilities|ToObject(Interface) _objecttointeract)
    (:Is%20Valid
      (Default|Interact _objecttointeract _charref))))

(fn GroundDetection
  (bind _charref (Variables|Default|GetcharRef))
  (bind _hashit (Default|SwimSpheretraceDiveStart _charref))
  (if _hashit
    (Default|ChangeCurrentState _charref "/Game/Assets/AmplifyAnimationPack/Blueprints/Character/CharacterStates/BP_GroundedState.BP_GroundedState_C")))