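; Character state for falling in the Amplify Animation Pack's character state machine.
; On entry it resizes the capsule, offsets the mesh, adjusts camera lag and switches movement to Falling.
; Each update reads a landing linetrace, changing to the swim state over water or passing landing readiness and zero speed to the animation communicator.
; Attack input sets a combat action for one weapon type, unless the plunge-water trace returns true.
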(fn UpdateState
  (params (deltaTime :type Float%20%28single-precision%29))
  (bind _charref (Variables|Default|GetcharRef))
  (bind _charref_2 (Variables|Default|GetcharRef))
  (bind _charanimcommunicator (Variables|/Game/Assets/AmplifyAnimationPack/Blueprints/Character/BP_Character.BP_Character_C|GetcharAnimCommunicator _charref_2))
  (|CallParentFunction 0.0)
  (bind (_canland _iswater) (Default|FallingLinetraceDetector _charref))
  (if (and _canland _iswater)
    (Default|ChangeCurrentState (Variables|Default|GetcharRef) "/Game/Assets/AmplifyAnimationPack/Blueprints/Character/CharacterStates/BP_SwimState.BP_SwimState_C")
    (else
      (Default|SetCanLandVal _charanimcommunicator (or _canland (== (.z (Transformation|GetVelocity _charref)) 0.0)))
      (if true
        (Default|SetSpeedVal _charanimcommunicator 0.0)
        (else
          (return))))))

(fn EnterState
  (params (prevStateClass :type BP%20Character%20State%20Base%20Class%20Reference))
  (bind _charref (Variables|Default|GetcharRef))
  (bind _charref_2 (Variables|Default|GetcharRef))
  (bind _charref_3 (Variables|Default|GetcharRef))
  (bind _charanimcommunicator (Variables|/Game/Assets/AmplifyAnimationPack/Blueprints/Character/BP_Character.BP_Character_C|GetcharAnimCommunicator _charref_2))
  (|CallParentFunction 0)
  (Components|Capsule|SetCapsuleHalfHeight (Variables|/Script/Engine.Character|GetCapsuleComponent _charref_3) 75.0 true)
  (Transformation|SetRelativeLocation (Variables|/Script/Engine.Character|GetMesh _charref_3) "0, 0,-75.000000" false false)
  (Variables|/Script/Engine.SpringArmComponent|SetCameraLagSpeed (Variables|/Game/Assets/AmplifyAnimationPack/Blueprints/Character/BP_Character.BP_Character_C|GetCameraArm _charref_2) (Variables|/Game/Assets/AmplifyAnimationPack/Blueprints/Character/BP_Character.BP_Character_C|GetcameraLagSpeedHeightFactor _charref_3))
  (Default|SetCanLandVal _charanimcommunicator false)
  (Default|SetMovementStateVal _charanimcommunicator "NewEnumerator8")
  (Pawn|Components|CharacterMovement|SetMovementMode (Variables|/Script/Engine.Character|GetCharacterMovement _charref) "MOVE_Falling" 0)
  (Default|SetNewCapsuleRadius _charref 3e+01 0.0))

(fn InputAttack
  (params (AttackState :type Character_CombatAction_Enum%20Enum :default "NewEnumerator0"))
  (bind _charref (Variables|Default|GetcharRef))
  (|CallParentFunction "NewEnumerator0")
  (bind _curentvalue (Default|GetWeaponTypeVal (Variables|/Game/Assets/AmplifyAnimationPack/Blueprints/Character/BP_Character.BP_Character_C|GetcharAnimCommunicator (Variables|Default|GetcharRef))))
  (if (Utilities|Enum|Equal(Enum) _curentvalue "NewEnumerator0")
    (bind _hashitwater (Default|PlungeWaterLinetrace _charref))
    (if (not _hashitwater)
      (Default|SetCombatActionVal (Variables|/Game/Assets/AmplifyAnimationPack/Blueprints/Character/BP_Character.BP_Character_C|GetcharAnimCommunicator _charref) AttackState))
    (else
      (return))))