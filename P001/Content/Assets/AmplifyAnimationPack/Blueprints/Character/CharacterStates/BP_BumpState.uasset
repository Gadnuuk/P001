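; BP_BumpState is a character state in the Amplify Animation Pack, apparently for when the character bumps into something.
; On entry it runs the parent logic, then zeroes the speed value and sets the movement state through the character's animation communicator.
; Interact input still works here: after the parent handler, it calls Interact on the character's ObjectToInteract if that reference is valid.
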(fn EnterState
  (params (prevStateClass :type BP%20Character%20State%20Base%20Class%20Reference))
  (bind _charref (Variables|Default|GetcharRef))
  (bind _charanimcommunicator (Variables|/Game/Assets/AmplifyAnimationPack/Blueprints/Character/BP_Character.BP_Character_C|GetcharAnimCommunicator _charref))
  (|CallParentFunction 0)
  (Default|SetSpeedVal _charanimcommunicator 0.0)
  (Default|SetMovementStateVal _charanimcommunicator "NewEnumerator23"))

(fn InputInteract
  (bind _charref (Variables|Default|GetcharRef))
  (bind _objecttointeract (Variables|/Game/Assets/AmplifyAnimationPack/Blueprints/Character/BP_Character.BP_Character_C|GetobjectToInteract _charref))
  (|CallParentFunction)
  (Utilities|IsValid (Utilities|ToObject(Interface) _objecttointeract)
    (:Is%20Valid
      (Default|Interact _objecttointeract _charref))
    (:Is%20Not%20Valid
      (return))))