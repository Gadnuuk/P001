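; Character state for hanging from a BP_BarActor, driving shimmying, corner moves and exit actions.
; Entering sets flying movement, aligns the character to the bar's facing and position, and locks CanMove.
; Sideways input uses line and sphere traces to pick hang actions; jump, crouch and forward trigger other animation actions, while interact switches to falling.
; While movable, each update sphere-traces to keep the character facing the bar.
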(fn EnterState
  (params (prevStateClass :type BP%20Character%20State%20Base%20Class%20Reference))
  (bind _charref (Variables|Default|GetcharRef))
  (bind _charref_2 (Variables|Default|GetcharRef))
  (bind _charref_3 (Variables|Default|GetcharRef))
  (bind _returnvalue (Transformation|GetActorLocation _charref_3))
  (bind _returnvalue_2 (Transformation|GetActorRotation _charref_2))
  (bind _charanimcommunicator (Variables|/Game/Assets/AmplifyAnimationPack/Blueprints/Character/BP_Character.BP_Character_C|GetcharAnimCommunicator _charref))
  (|CallParentFunction 0)
  (Collision|SetCollisionEnabled (Variables|/Script/Engine.Character|GetCapsuleComponent _charref) "QueryOnly")
  (Pawn|Components|CharacterMovement|SetMovementMode (Variables|/Script/Engine.Character|GetCharacterMovement _charref) "MOVE_Flying" 0)
  (Default|SetMovementStateVal _charanimcommunicator "NewEnumerator21")
  (Default|SetBarHangActionVal _charanimcommunicator "NewEnumerator0")
  (Variables|Default|SetcanMove false)
  (bind _asbp_bar_actor (Utilities|Casting|CastToBP_BarActor (Variables|/Game/Assets/AmplifyAnimationPack/Blueprints/Character/BP_Character.BP_Character_C|GetobjectToInteract _charref_2)))
  (Default|AdjustRotation _charref_2 (Math|Rotator|GetRotationXVector (Math|Rotator|MakeRotator (.roll _returnvalue_2) (.pitch _returnvalue_2) (+ (.yaw (Transformation|GetActorRotation _asbp_bar_actor)) (* (Math|Float|SelectFloat 1.0 (Math|Float|Sign(Float) (- (Math|Float|SelectFloat -1.8e+02 (.yaw _returnvalue_2) (Math|Float|NearlyEqual(Float) (Math|Float|Absolute(Float) (.yaw _returnvalue_2)) 1.8e+02 0.01)) (.yaw (Transformation|GetActorRotation _asbp_bar_actor)))) (== (Math|Float|Sign(Float) (- (Math|Float|SelectFloat -1.8e+02 (.yaw _returnvalue_2) (Math|Float|NearlyEqual(Float) (Math|Float|Absolute(Float) (.yaw _returnvalue_2)) 1.8e+02 0.01)) (.yaw (Transformation|GetActorRotation _asbp_bar_actor)))) 0.0)) 9e+01)))) true 12.0)
  (bind _asbp_bar_actor_2 (Utilities|Casting|CastToBP_BarActor (Variables|/Game/Assets/AmplifyAnimationPack/Blueprints/Character/BP_Character.BP_Character_C|GetobjectToInteract _charref_3)))
  (Default|AdjustPosition (Variables|Default|GetcharRef) _returnvalue (- (+ (* (Transformation|GetActorForwardVector _asbp_bar_actor_2) (* (* (Math|Float|Sign(Float) (Math|Vector|DotProduct (Math|Vector|Normalize (Math|Vector|MakeVector (.x (- (Transformation|GetActorLocation _asbp_bar_actor_2) (Transformation|GetActorLocation _charref_3))) (.y (- (Transformation|GetActorLocation _asbp_bar_actor_2) (Transformation|GetActorLocation _charref_3))) 0.0)) (Transformation|GetActorForwardVector _asbp_bar_actor_2))) -1.0) (Math|Vector|VectorLength (Math|Vector|MakeVector (.x (- (Transformation|GetActorLocation _asbp_bar_actor_2) (Transformation|GetActorLocation _charref_3))) (.y (- (Transformation|GetActorLocation _asbp_bar_actor_2) (Transformation|GetActorLocation _charref_3))) 0.0)))) (Transformation|GetActorLocation _asbp_bar_actor_2) (* (Transformation|GetActorRightVector _asbp_bar_actor_2) (* (Math|Float|SelectFloat 1.0 (Math|Float|Sign(Float) (- (Math|Float|SelectFloat -1.8e+02 (.yaw _returnvalue_2) (Math|Float|NearlyEqual(Float) (Math|Float|Absolute(Float) (.yaw _returnvalue_2)) 1.8e+02 0.01)) (.yaw (Transformation|GetActorRotation _asbp_bar_actor)))) (== (Math|Float|Sign(Float) (- (Math|Float|SelectFloat -1.8e+02 (.yaw _returnvalue_2) (Math|Float|NearlyEqual(Float) (Math|Float|Absolute(Float) (.yaw _returnvalue_2)) 1.8e+02 0.01)) (.yaw (Transformation|GetActorRotation _asbp_bar_actor)))) 0.0)) -2e+01))) _returnvalue) false true true))

(fn InputMoveRight
  (params (inputVal :type Float%20%28single-precision%29))
  (bind _charref (Variables|Default|GetcharRef))
  (bind _charref_2 (Variables|Default|GetcharRef))
  (bind _charref_3 (Variables|Default|GetcharRef))
  (bind _charref_4 (Variables|Default|GetcharRef))
  (bind _charref_5 (Variables|Default|GetcharRef))
  (bind _charanimcommunicator (Variables|/Game/Assets/AmplifyAnimationPack/Blueprints/Character/BP_Character.BP_Character_C|GetcharAnimCommunicator _charref_2))
  (bind _charanimcommunicator_2 (Variables|/Game/Assets/AmplifyAnimationPack/Blueprints/Character/BP_Character.BP_Character_C|GetcharAnimCommunicator _charref_4))
  (|CallParentFunction 0.0)
  (if (Variables|Default|GetcanMove)
    (bind _output_get (Variables|/Game/Assets/AmplifyAnimationPack/Blueprints/Character/BP_Character.BP_Character_C|SetInputRight _charref_5 inputVal))
    (bind _currentval (Default|SetInputRightVal (Variables|/Game/Assets/AmplifyAnimationPack/Blueprints/Character/BP_Character.BP_Character_C|GetcharAnimCommunicator _charref_5) _output_get))
    (if (!= _currentval 0.0)
      (bind _ishitting (Default|BarHangLinetraceMovement _charref _currentval))
      (if _ishitting
        (bind _ishitting_2 (Default|BarHangSpheretraceCorner _charref_3 _currentval -1.0 55.0))
        (if _ishitting_2
          (Default|SetBarHangActionVal _charanimcommunicator "NewEnumerator4")
          (Variables|Default|SetcanMove false)
          (else
            (Default|SetBarHangActionVal _charanimcommunicator "NewEnumerator1")))
        (else
          (bind _ishitting_3 (Default|BarHangSpheretraceCorner _charref_3 _currentval -1.0 9e+01))
          (if _ishitting_3
            (Default|SetBarHangActionVal _charanimcommunicator_2 "NewEnumerator4")
            (Variables|Default|SetcanMove false)
            (else
              (bind _ishitting_4 (Default|BarHangSpheretraceCorner _charref_4 _currentval 1.0 0.0))
              (if _ishitting_4
                (Default|SetBarHangActionVal _charanimcommunicator_2 "NewEnumerator3")
                (else
                  (Default|SetBarHangActionVal _charanimcommunicator_2 "NewEnumerator0")))))))
      (else
        (Default|SetBarHangActionVal (Variables|/Game/Assets/AmplifyAnimationPack/Blueprints/Character/BP_Character.BP_Character_C|GetcharAnimCommunicator _charref) "NewEnumerator0")))
    (else
      (return))))

(fn InputInteract
  (|CallParentFunction)
  (if (Variables|Default|GetcanMove)
    (Default|ChangeCurrentState (Variables|Default|GetcharRef) "/Game/Assets/AmplifyAnimationPack/Blueprints/Character/CharacterStates/BP_FallingState.BP_FallingState_C")))

(fn InputCrouchHold
  (params (inputVal :type Float%20%28single-precision%29))
  (|CallParentFunction 0.0)
  (if (and (> inputVal 0.0) (Variables|Default|GetcanMove))
    (Default|SetBarHangActionVal (Variables|/Game/Assets/AmplifyAnimationPack/Blueprints/Character/BP_Character.BP_Character_C|GetcharAnimCommunicator (Variables|Default|GetcharRef)) "NewEnumerator7")
    (Variables|Default|SetcanMove false)))

(fn InputJump
  (bind _charref (Variables|Default|GetcharRef))
  (|CallParentFunction)
  (bind _ishitting (Default|BarHangLinetraceJump _charref))
  (if _ishitting
    (Variables|Default|SetcanMove false)
    (Default|SetBarHangActionVal (Variables|/Game/Assets/AmplifyAnimationPack/Blueprints/Character/BP_Character.BP_Character_C|GetcharAnimCommunicator _charref) "NewEnumerator9")))

(fn InputMoveForward
  (params (inputVal :type Float%20%28single-precision%29))
  (bind _charref (Variables|Default|GetcharRef))
  (bind _charanimcommunicator (Variables|/Game/Assets/AmplifyAnimationPack/Blueprints/Character/BP_Character.BP_Character_C|GetcharAnimCommunicator _charref))
  (|CallParentFunction 0.0)
  (if (and (> inputVal 0.0) (Variables|Default|GetcanMove))
    (Variables|Default|SetcanMove false)
    (Pawn|Components|CharacterMovement|SetMovementMode (Variables|/Script/Engine.Character|GetCharacterMovement _charref) "MOVE_Flying" 0)
    (Default|SetBarWalkActionVal _charanimcommunicator "NewEnumerator0")
    (Default|SetBarHangActionVal _charanimcommunicator "NewEnumerator10")
    (Default|SetSpeedVal _charanimcommunicator 0.0)))

(fn UpdateState
  (params (deltaTime :type Float%20%28single-precision%29))
  (bind _charref (Variables|Default|GetCharRef))
  (|CallParentFunction 0.0)
  (if (Variables|Default|GetcanMove)
    (bind (_result _ishitting) (Default|BarHangSpheretraceHangCheck _charref))
    (if _ishitting
      (Default|AdjustRotation _charref (Math|Rotator|GetRotationXVector (Math|Rotator|MakeRotator 0.0 0.0 (- (.yaw (Math|Conversions|RotationFromXVector (.ImpactNormal (Collision|BreakHitResult _result)))) 1.8e+02))) true 1e+01))))