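; Character state for a big climb, part of the Amplify Animation Pack's character state machine.
; On entry it sets flying movement, adjusts camera lag, faces the obstacle, resizes the capsule, nudges its position and signals the animation communicator.
; Each update traces for a hang start to switch to BP_HangState.
; A failed climb-maintain trace, exceeded time threshold or jump input all trigger the same hang action in animation.
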(fn UpdateState
  (params (deltaTime :type Float%20%28single-precision%29))
  (bind _charref (Variables|Default|GetcharRef))
  (bind _charref_2 (Variables|Default|GetcharRef))
  (|CallParentFunction 0.0)
  (bind _output_get (Variables|Default|SetClimbTimer (+ deltaTime (Variables|Default|GetClimbTimer))))
  (if (<= _output_get (Variables|/Game/Assets/AmplifyAnimationPack/Blueprints/Character/BP_Character.BP_Character_C|GetclimbingTimeThreshold _charref_2))
    (bind _ishitting (Default|ClimbLinetraceHangStart _charref))
    (if _ishitting
      (Default|ChangeCurrentState _charref "/Game/Assets/AmplifyAnimationPack/Blueprints/Character/CharacterStates/BP_HangState.BP_HangState_C")
      (else
        (bind _ishitting_2 (Default|ClimbLinetraceClimbMantain _charref_2))
        (if (not _ishitting_2)
          (Default|SetHangActionVal (Variables|/Game/Assets/AmplifyAnimationPack/Blueprints/Character/BP_Character.BP_Character_C|GetcharAnimCommunicator (Variables|Default|GetcharRef)) "NewEnumerator6"))))
    (else
      (Default|SetHangActionVal (Variables|/Game/Assets/AmplifyAnimationPack/Blueprints/Character/BP_Character.BP_Character_C|GetcharAnimCommunicator _charref_2) "NewEnumerator6"))))

(fn EnterState
  (params (prevStateClass :type BP%20Character%20State%20Base%20Class%20Reference))
  (bind _charref (Variables|Default|GetcharRef))
  (bind _charref_2 (Variables|Default|GetcharRef))
  (bind _charref_3 (Variables|Default|GetcharRef))
  (bind _charanimcommunicator (Variables|/Game/Assets/AmplifyAnimationPack/Blueprints/Character/BP_Character.BP_Character_C|GetcharAnimCommunicator _charref_2))
  (|CallParentFunction 0)
  (Variables|/Script/Engine.SpringArmComponent|SetCameraLagSpeed (Variables|/Game/Assets/AmplifyAnimationPack/Blueprints/Character/BP_Character.BP_Character_C|GetCameraArm _charref) (Variables|/Game/Assets/AmplifyAnimationPack/Blueprints/Character/BP_Character.BP_Character_C|GetcameraLagSpeedHeightFactor _charref))
  (Pawn|Components|CharacterMovement|SetMovementMode (Variables|/Script/Engine.Character|GetCharacterMovement _charref) "MOVE_Flying" 0)
  (Default|SetMovementStateVal _charanimcommunicator "NewEnumerator9")
  (Default|SetHangActionVal _charanimcommunicator "NewEnumerator0")
  (Default|AdjustRotation _charref_2 (* (Variables|/Game/Assets/AmplifyAnimationPack/Blueprints/Character/BP_Character.BP_Character_C|GetobjToInteractRotVector _charref_2) -1.0) false 0.0)
  (Default|SetNewCapsuleRadius _charref_3 3e+01 0.0)
  (Default|AdjustPosition _charref_3 (Transformation|GetActorLocation _charref_3) (* (Transformation|GetActorForwardVector _charref_3) 3e+01) true true false)
  (Variables|Default|SetClimbTimer 0.0))

(fn InputJump
  (|CallParentFunction)
  (Default|SetHangActionVal (Variables|/Game/Assets/AmplifyAnimationPack/Blueprints/Character/BP_Character.BP_Character_C|GetcharAnimCommunicator (Variables|Default|GetcharRef)) "NewEnumerator6"))