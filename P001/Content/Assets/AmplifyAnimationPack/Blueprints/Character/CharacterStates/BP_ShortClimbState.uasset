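; BP_ShortClimbState is a character state from the Amplify Animation Pack that handles the short climb.
; On entry it sets the animation communicator's movement state, zeroes its speed, switches movement to Flying and disables capsule and camera-arm collision.
; It also calls a 2D AdjustPosition using a short offset derived from the forward vector.
; On exit it restores Walking and both collision settings.
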(fn EnterState
  (params (prevStateClass :type BP%20Character%20State%20Base%20Class%20Reference))
  (bind _charref (Variables|Default|GetcharRef))
  (bind _charref_2 (Variables|Default|GetcharRef))
  (bind _returnvalue (Transformation|GetActorLocation _charref_2))
  (bind _charanimcommunicator (Variables|/Game/Assets/AmplifyAnimationPack/Blueprints/Character/BP_Character.BP_Character_C|GetcharAnimCommunicator _charref))
  (|CallParentFunction 0)
  (Variables|/Script/Engine.SpringArmComponent|SetbDoCollisionTest (Variables|/Game/Assets/AmplifyAnimationPack/Blueprints/Character/BP_Character.BP_Character_C|GetCameraArm _charref) false)
  (Default|SetMovementStateVal _charanimcommunicator "NewEnumerator7")
  (Default|SetSpeedVal _charanimcommunicator 0.0)
  (Pawn|Components|CharacterMovement|SetMovementMode (Variables|/Script/Engine.Character|GetCharacterMovement _charref) "MOVE_Flying" 0)
  (Collision|SetCollisionEnabled (Variables|/Script/Engine.Character|GetCapsuleComponent _charref) "NoCollision")
  (Default|AdjustPosition _charref_2 _returnvalue (- (+ (Transformation|GetActorLocation _charref_2) (* (Transformation|GetActorForwardVector _charref_2) 25.0)) _returnvalue) false false true))

(fn ExitState
  (bind _charref (Variables|Default|GetcharRef))
  (|CallParentFunction)
  (Pawn|Components|CharacterMovement|SetMovementMode (Variables|/Script/Engine.Character|GetCharacterMovement _charref) "MOVE_Walking" 0)
  (Variables|/Script/Engine.SpringArmComponent|SetbDoCollisionTest (Variables|/Game/Assets/AmplifyAnimationPack/Blueprints/Character/BP_Character.BP_Character_C|GetCameraArm _charref) true)
  (Collision|SetCollisionEnabled (Variables|/Script/Engine.Character|GetCapsuleComponent _charref) "QueryAndPhysics"))