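; Crawling state of the player character's state machine, handling movement, camera and weapon input while the character crawls.
; Entry shifts the character and camera down, and jump starts standing up if an overhead trace is clear.
; Movement input feeds the anim communicator, gated by a ground sphere trace, with sprint while moving sideways triggering an alternate movement state.
; Weapon actions require crawl idle, and low clearance lowers the camera offset smoothly.
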(fn EnterState
  (params (prevStateClass :type BP%20Character%20State%20Base%20Class%20Reference))
  (bind _charref (Variables|Default|GetcharRef))
  (bind _charref_2 (Variables|Default|GetcharRef))
  (bind _charref_3 (Variables|Default|GetcharRef))
  (bind _charref_4 (Variables|Default|GetcharRef))
  (bind _returnvalue (Transformation|GetActorLocation _charref_4))
  (bind _charanimcommunicator (Variables|/Game/Assets/AmplifyAnimationPack/Blueprints/Character/BP_Character.BP_Character_C|GetcharAnimCommunicator _charref))
  (|CallParentFunction 0)
  (Variables|Default|SetcanMove false)
  (Default|SetSpeedVal _charanimcommunicator 0.0)
  (Default|SetCrawlActionVal _charanimcommunicator "NewEnumerator14")
  (Default|SetMovementStateVal _charanimcommunicator "NewEnumerator12")
  (Variables|/Game/Assets/AmplifyAnimationPack/Blueprints/Character/BP_Character.BP_Character_C|SetcurrentRotationRate _charref_4 (Variables|/Game/Assets/AmplifyAnimationPack/Blueprints/Character/BP_Character.BP_Character_C|GetcrawlRotationRate _charref_4))
  (Default|CrawlAdjustCharacter _charref_4 true _returnvalue (- (+ _returnvalue (* (Transformation|GetActorUpVector _charref_4) -2e+01)) _returnvalue))
  (Variables|/Game/Assets/AmplifyAnimationPack/Blueprints/Character/BP_Character.BP_Character_C|SetcameraDistanceTarget _charref_2 (Variables|/Game/Assets/AmplifyAnimationPack/Blueprints/Character/BP_Character.BP_Character_C|GetcameraDistanceCrawl _charref_2))
  (Variables|/Game/Assets/AmplifyAnimationPack/Blueprints/Character/BP_Character.BP_Character_C|SetcameraHeightOffsetTarget _charref_2 (Variables|/Game/Assets/AmplifyAnimationPack/Blueprints/Character/BP_Character.BP_Character_C|GetcameraHeightOffsetCrawl _charref_2))
  (Variables|/Script/Engine.SpringArmComponent|SetProbeSize (Variables|/Game/Assets/AmplifyAnimationPack/Blueprints/Character/BP_Character.BP_Character_C|GetCameraArm _charref_2) 3e+01)
  (bind _curentvalue (Default|GetWeaponTypeVal (Variables|/Game/Assets/AmplifyAnimationPack/Blueprints/Character/BP_Character.BP_Character_C|GetcharAnimCommunicator _charref_3)))
  (if (Utilities|Enum|Equal(Enum) _curentvalue "NewEnumerator3")
    (Default|WeaponForceUnequip _charref_3)))

(fn InputMoveForward
  (params (inputVal :type Float%20%28single-precision%29))
  (bind _charref (Variables|Default|GetcharRef))
  (|CallParentFunction 0.0)
  (bind _output_get (Variables|/Game/Assets/AmplifyAnimationPack/Blueprints/Character/BP_Character.BP_Character_C|SetInputForward _charref (Math|Float|SelectFloat inputVal 0.0 (Variables|Default|GetcanMove))))
  (bind _currentval (Default|SetInputFwdVal (Variables|/Game/Assets/AmplifyAnimationPack/Blueprints/Character/BP_Character.BP_Character_C|GetcharAnimCommunicator _charref) _output_get))
  (Pawn|Input|AddMovementInput _charref (Math|Vector|GetForwardVector (Math|Rotator|MakeRotator 0.0 0.0 (.Yaw (Math|Rotator|BreakRotator (Pawn|GetControlRotation _charref :!class /Script/Engine.Pawn))))) (Math|Float|SelectFloat _currentval 0.0 (Variables|Default|GetcanMoveInDirection)) false))

(fn InputMoveRight
  (params (inputVal :type Float%20%28single-precision%29))
  (bind _charref (Variables|Default|GetcharRef))
  (|CallParentFunction 0.0)
  (bind _output_get (Variables|/Game/Assets/AmplifyAnimationPack/Blueprints/Character/BP_Character.BP_Character_C|SetInputRight _charref (Math|Float|SelectFloat inputVal 0.0 (Variables|Default|GetcanMove))))
  (bind _currentval (Default|SetInputRightVal (Variables|/Game/Assets/AmplifyAnimationPack/Blueprints/Character/BP_Character.BP_Character_C|GetcharAnimCommunicator _charref) _output_get))
  (Pawn|Input|AddMovementInput _charref (Math|Vector|GetRightVector (Math|Rotator|MakeRotator 0.0 0.0 (.Yaw (Math|Rotator|BreakRotator (Pawn|GetControlRotation _charref :!class /Script/Engine.Pawn))))) (Math|Float|SelectFloat _currentval 0.0 (Variables|Default|GetcanMoveInDirection)) false))

(fn UpdateStateAnimation
  (bind _charref (Variables|Default|GetcharRef))
  (bind _charref_2 (Variables|Default|GetcharRef))
  (bind _charref_3 (Variables|Default|GetcharRef))
  (bind _charref_4 (Variables|Default|GetcharRef))
  (bind _charref_5 (Variables|Default|GetcharRef))
  (bind _charanimcommunicator (Variables|/Game/Assets/AmplifyAnimationPack/Blueprints/Character/BP_Character.BP_Character_C|GetcharAnimCommunicator _charref_5))
  (bind _charanimcommunicator_2 (Variables|/Game/Assets/AmplifyAnimationPack/Blueprints/Character/BP_Character.BP_Character_C|GetcharAnimCommunicator _charref_4))
  (|CallParentFunction)
  (bind _curentvalue (Default|GetInputRightVal _charanimcommunicator_2))
  (bind _curentvalue_2 (Default|GetInputFwdVal _charanimcommunicator_2))
  (bind _curentvalue_3 (Default|GetCrawlActionVal _charanimcommunicator_2))
  (if (and (Utilities|Enum|Equal(Enum) _curentvalue_3 "NewEnumerator15") (Variables|Default|GetcanMove))
    (bind _curentvalue_4 (Default|GetMovementStateVal (Variables|/Game/Assets/AmplifyAnimationPack/Blueprints/Character/BP_Character.BP_Character_C|GetcharAnimCommunicator (Variables|Default|GetcharRef))))
    (if (or (Utilities|Enum|Equal(Enum) _curentvalue_4 "NewEnumerator12") (Utilities|Enum|Equal(Enum) _curentvalue_4 "NewEnumerator13"))
      (bind _currentvalue (Default|SetSpeedVal (Variables|/Game/Assets/AmplifyAnimationPack/Blueprints/Character/BP_Character.BP_Character_C|GetcharAnimCommunicator (Variables|Default|GetcharRef)) (Math|Float|Clamp(Float) (+ (Math|Float|Absolute(Float) _curentvalue) (Math|Float|Absolute(Float) _curentvalue_2)) -1.0)))
      (bind _newdirection (Default|UpdateDirection _charref (Variables|Default|GetisBackwards)))
      (Default|SetDirectionVal (Variables|/Game/Assets/AmplifyAnimationPack/Blueprints/Character/BP_Character.BP_Character_C|GetcharAnimCommunicator _charref) _newdirection)
      (if (> _currentvalue 0.0)
        (bind _isgrounded (Default|GroundCrawlingSpheretraceDetector _charref_3))
        (bind _output_get (Variables|Default|SetcanMoveInDirection _isgrounded))
        (if (not _output_get)
          (Default|SetSpeedVal (Variables|/Game/Assets/AmplifyAnimationPack/Blueprints/Character/BP_Character.BP_Character_C|GetcharAnimCommunicator _charref_3) 0.0))))
    (else
      (bind _curentvalue_5 (Default|GetMovementStateVal _charanimcommunicator))
      (if (Utilities|Enum|Equal(Enum) _curentvalue_5 "NewEnumerator13")
        (Default|SetSpeedVal _charanimcommunicator (Math|Float|Clamp(Float) (+ (Math|Float|Absolute(Float) _curentvalue) (Math|Float|Absolute(Float) _curentvalue_2)) -1.0))
        (bind _newdirection_2 (Default|UpdateDirection _charref_2 false))
        (Default|SetDirectionVal (Variables|/Game/Assets/AmplifyAnimationPack/Blueprints/Character/BP_Character.BP_Character_C|GetcharAnimCommunicator _charref_2) _newdirection_2)
        (else
          (Default|SetSpeedVal _charanimcommunicator 0.0)
          (return))))))

(fn InputJump
  (bind _charref (Variables|Default|GetcharRef))
  (bind _charref_2 (Variables|Default|GetcharRef))
  (bind _charref_3 (Variables|Default|GetcharRef))
  (bind _returnvalue (Transformation|GetActorLocation _charref))
  (bind _charanimcommunicator (Variables|/Game/Assets/AmplifyAnimationPack/Blueprints/Character/BP_Character.BP_Character_C|GetcharAnimCommunicator _charref_3))
  (|CallParentFunction)
  (bind _curentvalue (Default|GetCrawlActionVal (Variables|/Game/Assets/AmplifyAnimationPack/Blueprints/Character/BP_Character.BP_Character_C|GetcharAnimCommunicator (Variables|Default|GetcharRef))))
  (if (and (Variables|Default|GetcanMove) (Utilities|Enum|Equal(Enum) _curentvalue "NewEnumerator15"))
    (bind _canstand (Default|CanStandSpheretraceDetector _charref_3 4e+01))
    (if _canstand
      (Default|SetCrawlActionVal _charanimcommunicator "NewEnumerator16")
      (Default|SetSpeedVal _charanimcommunicator 0.0)
      (Default|CrawlAdjustCharacter _charref false _returnvalue (- (+ _returnvalue (* (Transformation|GetActorUpVector _charref) 35.0)) _returnvalue))
      (Variables|/Game/Assets/AmplifyAnimationPack/Blueprints/Character/BP_Character.BP_Character_C|SetcameraDistanceTarget _charref_2 (Variables|/Game/Assets/AmplifyAnimationPack/Blueprints/Character/BP_Character.BP_Character_C|GetcameraDistanceDefault _charref_2))
      (Variables|/Game/Assets/AmplifyAnimationPack/Blueprints/Character/BP_Character.BP_Character_C|SetcameraHeightOffsetTarget _charref_2 (Variables|/Game/Assets/AmplifyAnimationPack/Blueprints/Character/BP_Character.BP_Character_C|GetcameraHeightOffsetDefault _charref_2))
      (Variables|/Script/Engine.SpringArmComponent|SetTargetOffset (Variables|/Game/Assets/AmplifyAnimationPack/Blueprints/Character/BP_Character.BP_Character_C|GetCameraArm _charref_2) (Math|Vector|MakeVector 0.0 0.0 0.0))
      (Variables|Default|SetcanMove false))
    (else
      (return))))

(fn InputSprintHold
  (params (inputVal :type Float%20%28single-precision%29))
  (bind _charref (Variables|Default|GetcharRef))
  (bind _charanimcommunicator (Variables|/Game/Assets/AmplifyAnimationPack/Blueprints/Character/BP_Character.BP_Character_C|GetcharAnimCommunicator _charref))
  (|CallParentFunction 0.0)
  (if (Variables|Default|GetcanMove)
    (bind _curentvalue (Default|GetSpeedVal _charanimcommunicator))
    (bind _curentvalue_2 (Default|GetTargetDirectionVal _charanimcommunicator))
    (if (Math|Boolean|ANDBoolean (!= inputVal 0.0) (!= _curentvalue 0.0) (> (Math|Float|Absolute(Float) _curentvalue_2) 65.0) (< (Math|Float|Absolute(Float) _curentvalue_2) 135.0))
      (Default|SetMovementStateVal (Variables|/Game/Assets/AmplifyAnimationPack/Blueprints/Character/BP_Character.BP_Character_C|GetcharAnimCommunicator (Variables|Default|GetcharRef)) "NewEnumerator13")
      (Variables|Default|SetcanMove false)
      (Default|WeaponToggleAim (Variables|Default|GetcharRef) false)
      (else
        (bind _curentvalue_3 (Default|GetMovementStateVal (Variables|/Game/Assets/AmplifyAnimationPack/Blueprints/Character/BP_Character.BP_Character_C|GetcharAnimCommunicator (Variables|Default|GetcharRef))))
        (if (Utilities|Enum|Equal(Enum) _curentvalue_3 "NewEnumerator13")
          (Default|SetMovementStateVal (Variables|/Game/Assets/AmplifyAnimationPack/Blueprints/Character/BP_Character.BP_Character_C|GetcharAnimCommunicator (Variables|Default|GetcharRef)) "NewEnumerator12"))))
    (else
      (return))))

(fn UpdateState
  (params (deltaTime :type Float%20%28single-precision%29))
  (|CallParentFunction 0.0)
  (Default|RotateCharacter (Variables|Default|GetcharRef) (Variables|Default|GetcanMove) (Variables|Default|GetisBackwards))
  (CallFunction|LimitCameraTargetOffset deltaTime))

(fn ExitState
  (bind _charref (Variables|Default|GetcharRef))
  (bind _charanimcommunicator (Variables|/Game/Assets/AmplifyAnimationPack/Blueprints/Character/BP_Character.BP_Character_C|GetcharAnimCommunicator _charref))
  (|CallParentFunction)
  (Variables|/Script/Engine.CharacterMovementComponent|SetbAllowPhysicsRotationDuringAnimRootMotion (Variables|/Script/Engine.Character|GetCharacterMovement _charref) true)
  (Default|SetCrawlActionVal _charanimcommunicator "NewEnumerator14")
  (Default|SetLocomotionPrevStateVal _charanimcommunicator "NewEnumerator0")
  (Variables|/Script/Engine.SpringArmComponent|SetProbeSize (Variables|/Game/Assets/AmplifyAnimationPack/Blueprints/Character/BP_Character.BP_Character_C|GetCameraArm _charref) 12.0))

(fn InputWeaponShoot
  (bind _charref (Variables|Default|GetcharRef))
  (bind _charref_2 (Variables|Default|GetcharRef))
  (bind _charanimcommunicator (Variables|/Game/Assets/AmplifyAnimationPack/Blueprints/Character/BP_Character.BP_Character_C|GetcharAnimCommunicator _charref_2))
  (|CallParentFunction)
  (bind _curentvalue (Default|GetCrawlActionVal _charanimcommunicator))
  (bind _curentvalue_2 (Default|GetMovementStateVal _charanimcommunicator))
  (if (and (Utilities|IsCharacterinCrawlIdle _curentvalue _curentvalue_2) (Utilities|IsValid (Variables|/Game/Assets/AmplifyAnimationPack/Blueprints/Character/BP_Character.BP_Character_C|GetcurrentWeapon (Variables|Default|GetcharRef))))
    (bind _shotsuccesful (Default|WeaponStartShooting _charref))
    (if _shotsuccesful
      (Variables|Default|SetcanMove false)
      (Default|SetSpeedVal (Variables|/Game/Assets/AmplifyAnimationPack/Blueprints/Character/BP_Character.BP_Character_C|GetcharAnimCommunicator _charref) 0.0))))

(fn InputWeaponShootReleased
  (bind _charref (Variables|Default|GetcharRef))
  (bind _charref_2 (Variables|Default|GetcharRef))
  (bind _is_aiming (Variables|/Game/Assets/AmplifyAnimationPack/Blueprints/Character/BP_Character.BP_Character_C|GetIs%20Aiming _charref_2))
  (bind _charanimcommunicator (Variables|/Game/Assets/AmplifyAnimationPack/Blueprints/Character/BP_Character.BP_Character_C|GetcharAnimCommunicator _charref))
  (|CallParentFunction)
  (bind _curentvalue (Default|GetWeaponTypeVal _charanimcommunicator))
  (bind _curentvalue_2 (Default|GetWeaponActionVal _charanimcommunicator))
  (if (and (Utilities|Enum|NotEqual(Enum) _curentvalue "NewEnumerator0") (Utilities|Enum|Equal(Enum) _curentvalue_2 "NewEnumerator1"))
    (Default|SetWeaponActionVal (Variables|/Game/Assets/AmplifyAnimationPack/Blueprints/Character/BP_Character.BP_Character_C|GetcharAnimCommunicator _charref_2) (select _is_aiming "NewEnumerator3" "NewEnumerator0"))
    (Variables|Default|SetcanMove (not _is_aiming))))

(fn InputWeaponAim
  (bind _charref (Variables|Default|GetcharRef))
  (bind _charanimcommunicator (Variables|/Game/Assets/AmplifyAnimationPack/Blueprints/Character/BP_Character.BP_Character_C|GetcharAnimCommunicator _charref))
  (|CallParentFunction)
  (bind _curentvalue (Default|GetCrawlActionVal _charanimcommunicator))
  (bind _curentvalue_2 (Default|GetMovementStateVal _charanimcommunicator))
  (if (and (Utilities|IsCharacterinCrawlIdle _curentvalue _curentvalue_2) (Utilities|IsValid (Variables|/Game/Assets/AmplifyAnimationPack/Blueprints/Character/BP_Character.BP_Character_C|GetcurrentWeapon _charref)))
    (Default|WeaponToggleAim (Variables|Default|GetcharRef) true)))

(fn InputWeaponAimReleased
  (bind _charref (Variables|Default|GetcharRef))
  (bind _charanimcommunicator (Variables|/Game/Assets/AmplifyAnimationPack/Blueprints/Character/BP_Character.BP_Character_C|GetcharAnimCommunicator _charref))
  (|CallParentFunction)
  (bind _curentvalue (Default|GetWeaponTypeVal _charanimcommunicator))
  (bind _curentvalue_2 (Default|GetWeaponActionVal _charanimcommunicator))
  (if (and (Utilities|Enum|NotEqual(Enum) _curentvalue "NewEnumerator0") (or (Utilities|Enum|Equal(Enum) _curentvalue_2 "NewEnumerator3") (Utilities|Enum|Equal(Enum) _curentvalue_2 "NewEnumerator1")))
    (Default|WeaponToggleAim (Variables|Default|GetcharRef) false)))

(fn InputWeaponReload
  (bind _charref (Variables|Default|GetcharRef))
  (bind _charanimcommunicator (Variables|/Game/Assets/AmplifyAnimationPack/Blueprints/Character/BP_Character.BP_Character_C|GetcharAnimCommunicator _charref))
  (|CallParentFunction)
  (bind _curentvalue (Default|GetCrawlActionVal _charanimcommunicator))
  (bind _curentvalue_2 (Default|GetMovementStateVal _charanimcommunicator))
  (if (and (Utilities|IsCharacterinCrawlIdle _curentvalue _curentvalue_2) (Utilities|IsValid (Variables|/Game/Assets/AmplifyAnimationPack/Blueprints/Character/BP_Character.BP_Character_C|GetcurrentWeapon _charref)))
    (Default|WeaponReload (Variables|Default|GetcharRef))))

(fn InputWeaponEquip
  (bind _charref (Variables|Default|GetcharRef))
  (bind _charanimcommunicator (Variables|/Game/Assets/AmplifyAnimationPack/Blueprints/Character/BP_Character.BP_Character_C|GetcharAnimCommunicator _charref))
  (|CallParentFunction)
  (bind _curentvalue (Default|GetCrawlActionVal _charanimcommunicator))
  (bind _curentvalue_2 (Default|GetMovementStateVal _charanimcommunicator))
  (if (Utilities|IsCharacterinCrawlIdle _curentvalue _curentvalue_2)
    (Default|WeaponChangeWeapon (Variables|Default|GetcharRef))))

(fn LimitCameraTargetOffset
  (params (deltaTime :type Float%20%28single-precision%29))
  (bind _charref (Variables|Default|GetcharRef))
  (bind _cameraarm (Variables|/Game/Assets/AmplifyAnimationPack/Blueprints/Character/BP_Character.BP_Character_C|GetCameraArm _charref))
  (bind _canstand (Default|CanStandSpheretraceDetector _charref 4e+01))
  (Variables|/Script/Engine.SpringArmComponent|SetTargetOffset _cameraarm (Math|Vector|MakeVector (.x (Variables|/Script/Engine.SpringArmComponent|GetTargetOffset _cameraarm)) (.y (Variables|/Script/Engine.SpringArmComponent|GetTargetOffset _cameraarm)) (Math|Interpolation|FInterpTo (.z (Variables|/Script/Engine.SpringArmComponent|GetTargetOffset _cameraarm)) (Math|Float|SelectFloat 0.0 -55.0 _canstand) deltaTime 1e+01))))