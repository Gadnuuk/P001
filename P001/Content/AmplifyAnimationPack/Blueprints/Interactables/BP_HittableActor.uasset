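; BP_HittableActor is an interactable target that blows up when anything overlaps its HurtBox.
; The blow-up disables HurtBox and Cube collision, hides the cube and spawns the NS_HittableFX Niagara effect at its location, without destroying the actor.
; If the overlapping actor is a BP_Character, it removes this target from that character's possible lock-on actors and calls LockTriggerLockon when the character is locked.
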(event OnComponentBeginOverlap(HurtBox)
  (params (OverlappedComponent :type Primitive%20Component%20Object%20Reference) (OtherActor :type Actor%20Object%20Reference) (OtherComp :type Primitive%20Component%20Object%20Reference) (OtherBodyIndex :type Integer) (bFromSweep :type Boolean) (SweepResult :type Hit%20Result%20Structure%20%28by%20ref%29))
  (CallFunction|HittableBlowUp)
  (bind _asbp_character (Utilities|Casting|CastToBP_Character OtherActor))
  (Default|LockRemovePossibleActor _asbp_character self)
  (if (Variables|/Game/AmplifyAnimationPack/Blueprints/Character/BP_Character.BP_Character_C|GetisLocked _asbp_character)
    (Default|LockTriggerLockon _asbp_character)))

(fn ConstructionScript)

(fn HittableBlowUp
  (bind _cube (Variables|Default|GetCube))
  (Collision|SetCollisionEnabled (Variables|Default|GetHurtBox) "NoCollision")
  (Collision|SetCollisionEnabled _cube "NoCollision")
  (Rendering|SetVisibility _cube false false)
  (Niagara|SpawnSystematLocation "/Game/AmplifyAnimationPack/FX/NS_HittableFX.NS_HittableFX" (Transformation|GetWorldLocation _cube)))