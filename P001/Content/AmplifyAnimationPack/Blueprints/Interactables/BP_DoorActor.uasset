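; Interactable door that the player character can open and close, starting closed.
; A detector overlap registers the door as the character's interaction target and toggles the UI prompt.
; Interact puts the player in the interaction state, aligns them to their side of the door and selects an interaction animation type from side and door state.
; Separate Open and Close functions play the mesh animation, update IsClosed and toggle collision.
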(event OnComponentBeginOverlap(Player_Detector)
  (params (OverlappedComponent :type Primitive%20Component%20Object%20Reference) (OtherActor :type Actor%20Object%20Reference) (OtherComp :type Primitive%20Component%20Object%20Reference) (OtherBodyIndex :type Integer) (bFromSweep :type Boolean) (SweepResult :type Hit%20Result%20Structure%20%28by%20ref%29))
  ;[1 1 1] Player Detection
  (bind _asbp_character (Utilities|Casting|CastToBP_Character OtherActor))
  (Variables|/Game/AmplifyAnimationPack/Blueprints/Character/BP_Character.BP_Character_C|SetobjectToInteract _asbp_character self)
  (Default|UIShowInteractionUI _asbp_character "Press E to Open/Close Door"))

(event OnComponentEndOverlap(Player_Detector)
  (params (OverlappedComponent :type Primitive%20Component%20Object%20Reference) (OtherActor :type Actor%20Object%20Reference) (OtherComp :type Primitive%20Component%20Object%20Reference) (OtherBodyIndex :type Integer))
  ;[1 1 1] Player Detection
  (bind _asbp_character (Utilities|Casting|CastToBP_Character OtherActor))
  (Variables|/Game/AmplifyAnimationPack/Blueprints/Character/BP_Character.BP_Character_C|SetobjectToInteract _asbp_character 0)
  (Default|UIHideInteractionUI _asbp_character))

(event EventInteract
  (params (player :type BP%20Character%20Object%20Reference))
  (bind _returnvalue (Transformation|GetActorLocation player))
  (bind _signofside (Utilities|GetWhichSidePlayerIson player))
  (bind _playerposition (Variables|Default|GetPlayerPosition))
  (bind _returnvalue_2 (>= _signofside 0.0))
  (Default|ChangeCurrentState player "/Game/AmplifyAnimationPack/Blueprints/Character/CharacterStates/BP_InteractionState.BP_InteractionState_C")
  (Default|AdjustPosition player _returnvalue (- (Math|Vector|MakeVector (+ (.x (Transformation|GetActorLocation)) (* (.x (Transformation|GetActorForwardVector)) (* (.x (Variables|/Script/Engine.SceneComponent|GetRelativeLocation _playerposition)) _signofside))) (.y (Transformation|GetWorldLocation _playerposition)) (.z (Transformation|GetActorLocation player))) _returnvalue) false false true)
  (Default|AdjustRotation player (Math|Rotator|GetRotationXVector (Math|Rotator|MakeRotator 0.0 0.0 (+ (.yaw (Transformation|GetWorldRotation (Variables|Default|GetMesh))) (* 9e+01 _signofside)))) true 1e+01)
  (Default|SetInteractionTypeVal (Variables|/Game/AmplifyAnimationPack/Blueprints/Character/BP_Character.BP_Character_C|GetcharAnimCommunicator player) (select (Variables|Default|GetisClosed) (select _returnvalue_2 "NewEnumerator12" "NewEnumerator15") (select _returnvalue_2 "NewEnumerator13" "NewEnumerator16"))))

(event EventBeginPlay
  (Variables|Default|SetisClosed true))

(fn ConstructionScript)

(fn Open
  (Components|Animation|PlayAnimation (Variables|Default|GetMesh) "/Game/AmplifyAnimationPack/Animations/Interactables/Door_Open_Anim.Door_Open_Anim" false)
  (Variables|Default|SetisClosed false)
  (Collision|SetCollisionEnabled (Variables|Default|GetCollision) "NoCollision"))

(fn Close
  (Components|Animation|PlayAnimation (Variables|Default|GetMesh) "/Game/AmplifyAnimationPack/Animations/Interactables/Door_Close_Anim.Door_Close_Anim" false)
  (Variables|Default|SetisClosed true)
  (Collision|SetCollisionEnabled (Variables|Default|GetCollision) "QueryAndPhysics"))

(fn CheckResetPlayerCrouch
  (return true))