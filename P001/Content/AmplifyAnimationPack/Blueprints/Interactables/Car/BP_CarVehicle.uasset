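; Drivable car interactable that switches the interacting player into BP_CarState and takes over as the controlled vehicle.
; On possession it attaches the character with capsule collision off, then feeds input to throttle, steering and a pitch-clamped camera arm.
; Interacting again applies the handbrake, zeroes physics velocities and forwards the input to the car state.
; Door animations play on the side reported by the character's animation communicator.
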(event EventInteract
  (params (player :type BP%20Character%20Object%20Reference))
  ;[1 1 1] Interaction begin event
  (Default|ChangeCurrentState player "/Game/AmplifyAnimationPack/Blueprints/Character/CharacterStates/BP_CarState.BP_CarState_C")
  (Default|UIHideInteractionUI player)
  (Variables|Default|SetplayerChar player)
  (Transformation|SetRelativeRotation (Variables|Default|GetCameraArm) "0, 0, 0" false false))

(event EventInputPossessEvent
  (bind _playerchar (Variables|Default|GetplayerChar))
  ;[1 1 1] Possession Event
  (Transformation|AttachActorToActor _playerchar self "None" "KeepWorld" "KeepWorld" "KeepWorld" false)
  (Collision|SetCollisionEnabled (Variables|/Script/Engine.Character|GetCapsuleComponent _playerchar) "NoCollision")
  (Variables|Default|SetcanMove true)
  (Variables|Default|SetcanMoveCamera true))

(event EventMoveRightInputEvent
  (params (valueAxis :type Float%20%28single-precision%29))
  ;[1 1 1] Input Axis
  (if (Variables|Default|GetcanMove)
    (Class|WheeledVehicleMovementComponent|SetSteeringInput (Variables|Default|GetVehicleMovement) valueAxis)))

(event EventInteractInputEvent
  (bind _vehiclemovement (Variables|Default|GetVehicleMovement))
  (bind _updatedprimitive (Variables|/Script/Engine.MovementComponent|GetUpdatedPrimitive _vehiclemovement))
  ;[1 1 1] Input Actions
  (Variables|Default|SetcanMove false)
  (Variables|Default|SetcanMoveCamera false)
  (Class|WheeledVehicleMovementComponent|SetHandbrakeInput _vehiclemovement true)
  (Class|PrimitiveComponent|SetAllPhysicsLinearVelocity _updatedprimitive "0, 0, 0" false)
  (Class|PrimitiveComponent|SetAllPhysicsAngularVelocityinDegrees _updatedprimitive (Math|Vector|VectorZero) false)
  (bind _asbp_car_state (Utilities|Casting|CastToBP_CarState (Variables|/Game/AmplifyAnimationPack/Blueprints/Character/BP_Character.BP_Character_C|GetcurrentState (Variables|Default|GetplayerChar))))
  (Default|InputInteract _asbp_car_state))

(event EventLookUpInputEvent
  (params (valueInput :type Float%20%28single-precision%29))
  (bind _cameraarm (Variables|Default|GetCameraArm))
  (bind _relativerotation (Variables|/Script/Engine.SceneComponent|GetRelativeRotation _cameraarm))
  ;[1 1 1] Input Axis
  (if (Variables|Default|GetcanMoveCamera)
    (Transformation|SetRelativeRotation _cameraarm (Math|Rotator|MakeRotator 0.0 (Math|Float|Clamp(Float) (+ (.pitch _relativerotation) (* valueInput (select (Variables|/Game/AmplifyAnimationPack/Blueprints/Character/BP_Character.BP_Character_C|GetisYInverted (Variables|Default|GetplayerChar)) 1.0 -1.0))) -3e+01 3e+01) (.yaw _relativerotation)) false false)))

(event EventTurnInputEvent
  (params (valueInput :type Float%20%28single-precision%29))
  ;[1 1 1] Input Axis
  (if (Variables|Default|GetcanMoveCamera)
    (Transformation|AddRelativeRotation (Variables|Default|GetCameraArm) (Math|Rotator|MakeRotator 0.0 0.0 valueInput) false false)))

(event EventCarAccelerateInputEvent
  (params (valueInput :type Float%20%28single-precision%29))
  ;[1 1 1] Input Axis
  (if (Variables|Default|GetcanMove)
    (Class|WheeledVehicleMovementComponent|SetThrottleInput (Variables|Default|GetVehicleMovement) valueInput)))

(fn ConstructionScript)

(fn OpenDoor
  (bind _curentvalue (Default|GetCarDirVal (Variables|/Game/AmplifyAnimationPack/Blueprints/Character/BP_Character.BP_Character_C|GetcharAnimCommunicator (Variables|Default|GetplayerChar))))
  (Components|Animation|PlayAnimation (Variables|Character|GetMesh) (Utilities|Select :Index _curentvalue :NewEnumerator12 "/Game/AmplifyAnimationPack/Animations/Interactables/Car_R_Door_Anim.Car_R_Door_Anim" :NewEnumerator13 "/Game/AmplifyAnimationPack/Animations/Interactables/Car_L_Door_Anim.Car_L_Door_Anim") false))

(fn CheckResetPlayerCrouch
  (return true))