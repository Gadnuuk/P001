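; BP_BarActor is an interactable bar that the player character can climb and hang from.
; Its Player_Detector overlap registers the bar as the BP_Character's ObjectToInteract and shows a climb prompt, clearing both on exit.
; Interact switches the player into BP_BarHangState and hides the prompt, while CheckResetPlayerCrouch always returns false.
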(event OnComponentBeginOverlap(Player_Detector)
  (params (OverlappedComponent :type Primitive%20Component%20Object%20Reference) (OtherActor :type Actor%20Object%20Reference) (OtherComp :type Primitive%20Component%20Object%20Reference) (OtherBodyIndex :type Integer) (bFromSweep :type Boolean) (SweepResult :type Hit%20Result%20Structure%20%28by%20ref%29))
  (bind _asbp_character (Utilities|Casting|CastToBP_Character OtherActor))
  (Variables|/Game/AmplifyAnimationPack/Blueprints/Character/BP_Character.BP_Character_C|SetobjectToInteract _asbp_character self)
  (Default|UIShowInteractionUI _asbp_character "Press E to Climb Bar"))

(event OnComponentEndOverlap(Player_Detector)
  (params (OverlappedComponent :type Primitive%20Component%20Object%20Reference) (OtherActor :type Actor%20Object%20Reference) (OtherComp :type Primitive%20Component%20Object%20Reference) (OtherBodyIndex :type Integer))
  (bind _asbp_character (Utilities|Casting|CastToBP_Character OtherActor))
  (Variables|/Game/AmplifyAnimationPack/Blueprints/Character/BP_Character.BP_Character_C|SetobjectToInteract _asbp_character 0)
  (Default|UIHideInteractionUI _asbp_character))

(event EventInteract
  (params (player :type BP%20Character%20Object%20Reference))
  (Default|ChangeCurrentState player "/Game/AmplifyAnimationPack/Blueprints/Character/CharacterStates/BP_BarHangState.BP_BarHangState_C")
  (Default|UIHideInteractionUI player))

(fn ConstructionScript)

(fn CheckResetPlayerCrouch
  (return false))