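; Character state for vaulting in the Amplify Animation Pack, built on a parent state's enter, update and exit hooks.
; On enter it sets movement to Flying, passes vault type and movement state to the animation communicator, and saves the camera's maximum pitch.
; Each update smoothly interpolates that pitch limit toward zero, and exit restores the saved value.
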(fn EnterState
  (params (prevStateClass :type BP%20Character%20State%20Base%20Class%20Reference))
  (bind _charref (Variables|Default|GetcharRef))
  (bind _charanimcommunicator (Variables|/Game/AmplifyAnimationPack/Blueprints/Character/BP_Character.BP_Character_C|GetcharAnimCommunicator _charref))
  (|CallParentFunction 0)
  (Pawn|Components|CharacterMovement|SetMovementMode (Variables|/Script/Engine.Character|GetCharacterMovement _charref) "MOVE_Flying" 0)
  (Default|SetVaultTypeVal _charanimcommunicator "NewEnumerator0")
  (Default|SetMovementStateVal _charanimcommunicator "NewEnumerator22")
  (Variables|Default|SetprevCameraMaxPitchValue (Variables|/Game/AmplifyAnimationPack/Blueprints/Character/BP_Character.BP_Character_C|GetcameraPitchValueMax (Variables|Default|GetcharRef))))

(fn UpdateState
  (params (deltaTime :type Float%20%28single-precision%29))
  (bind _charref (Variables|Default|GetcharRef))
  (|CallParentFunction 0.0)
  (Variables|/Game/AmplifyAnimationPack/Blueprints/Character/BP_Character.BP_Character_C|SetcameraPitchValueMax _charref (Math|Interpolation|FInterpTo (Variables|/Game/AmplifyAnimationPack/Blueprints/Character/BP_Character.BP_Character_C|GetcameraPitchValueMax _charref) 0.0 deltaTime 7.0)))

(fn ExitState
  (|CallParentFunction)
  (Variables|/Game/AmplifyAnimationPack/Blueprints/Character/BP_Character.BP_Character_C|SetcameraPitchValueMax (Variables|Default|GetcharRef) (Variables|Default|GetprevCameraMaxPitchValue)))