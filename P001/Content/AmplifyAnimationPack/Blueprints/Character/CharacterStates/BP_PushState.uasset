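; Character state for pushing an object, part of the character state machine in the Amplify Animation Pack.
; On entry it stops movement, disables orient-to-movement, snaps the character to face opposite the interact object's rotation vector and reports the state to the anim communicator.
; Only non-negative forward input drives movement, along control yaw, and feeds the animation input value.
; Jump or Interact switches the communicator's movement state to end the push.
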(fn EnterState
  (params (prevStateClass :type BP%20Character%20State%20Base%20Class%20Reference))
  (bind _charref (Variables|Default|GetcharRef))
  (bind _charref_2 (Variables|Default|GetcharRef))
  (bind _charactermovement (Variables|/Script/Engine.Character|GetCharacterMovement _charref))
  (bind _charanimcommunicator (Variables|/Game/AmplifyAnimationPack/Blueprints/Character/BP_Character.BP_Character_C|GetcharAnimCommunicator _charref))
  (|CallParentFunction 0)
  (Components|Movement|StopMovementImmediately _charactermovement)
  (Default|SetSpeedVal _charanimcommunicator 0.0)
  (Variables|/Script/Engine.CharacterMovementComponent|SetbOrientRotationToMovement _charactermovement false)
  (Default|SetMovementStateVal _charanimcommunicator "NewEnumerator14")
  (Default|AdjustRotation _charref_2 (* (Variables|/Game/AmplifyAnimationPack/Blueprints/Character/BP_Character.BP_Character_C|GetobjToInteractRotVector _charref_2) -1.0) false 0.0))

(fn InputMoveForward
  (params (inputVal :type Float%20%28single-precision%29))
  (bind _charref (Variables|Default|GetcharRef))
  (|CallParentFunction 0.0)
  (if (>= inputVal 0.0)
    (bind _output_get (Variables|/Game/AmplifyAnimationPack/Blueprints/Character/BP_Character.BP_Character_C|SetInputForward _charref inputVal))
    (bind _currentval (Default|SetInputFwdVal (Variables|/Game/AmplifyAnimationPack/Blueprints/Character/BP_Character.BP_Character_C|GetcharAnimCommunicator _charref) _output_get))
    (Pawn|Input|AddMovementInput _charref (Math|Vector|GetForwardVector (Math|Rotator|MakeRotator 0.0 0.0 (.Yaw (Math|Rotator|BreakRotator (Pawn|GetControlRotation _charref :!class /Script/Engine.Pawn))))) _currentval false)))

(fn InputJump
  (|CallParentFunction)
  (Default|SetMovementStateVal (Variables|/Game/AmplifyAnimationPack/Blueprints/Character/BP_Character.BP_Character_C|GetcharAnimCommunicator (Variables|Default|GetcharRef)) "NewEnumerator0"))

(fn ExitState
  (|CallParentFunction))

(fn InputInteract
  (|CallParentFunction)
  (Default|SetMovementStateVal (Variables|/Game/AmplifyAnimationPack/Blueprints/Character/BP_Character.BP_Character_C|GetcharAnimCommunicator (Variables|Default|GetcharRef)) "NewEnumerator0"))