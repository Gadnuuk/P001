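; Character state for walking along the top of a BP_BarActor.
; On entry it stops movement and snaps the character onto the bar's axis, using dot products and the bar-hang action to pick facing and position.
; Movement inputs drive animation speed and direction through CharAnimCommunicator, while a ground sphere trace switches to grounded or falling state off the bar.
; Interact, when CanDrop allows, sets a bar-walk action that suspends these updates.
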(fn EnterState
  (params (prevStateClass :type BP%20Character%20State%20Base%20Class%20Reference))
  (bind _charref (Variables|Default|GetcharRef))
  (bind _charref_2 (Variables|Default|GetcharRef))
  (bind _charref_3 (Variables|Default|GetcharRef))
  (bind _charref_4 (Variables|Default|GetcharRef))
  (bind _returnvalue (Transformation|GetActorLocation _charref_3))
  (bind _charanimcommunicator (Variables|/Game/AmplifyAnimationPack/Blueprints/Character/BP_Character.BP_Character_C|GetcharAnimCommunicator _charref))
  (bind _charactermovement (Variables|/Script/Engine.Character|GetCharacterMovement _charref))
  (|CallParentFunction 0)
  (Components|Movement|StopMovementImmediately _charactermovement)
  (Pawn|Components|CharacterMovement|SetMovementMode _charactermovement "MOVE_Walking" 0)
  (Default|SetSpeedVal _charanimcommunicator 0.0)
  (Default|SetMovementStateVal _charanimcommunicator "NewEnumerator20")
  (Default|SetBarWalkActionVal _charanimcommunicator "NewEnumerator0")
  (bind _currentbaractor (CallFunction|CheckIsonBar))
  (Utilities|IsValid _currentbaractor
    (:Is%20Valid
      (bind _curentvalue (Default|GetBarHangActionVal (Variables|/Game/AmplifyAnimationPack/Blueprints/Character/BP_Character.BP_Character_C|GetcharAnimCommunicator (Variables|Default|GetcharRef))))
      (Default|AdjustRotation (Variables|Default|GetcharRef) (select (Utilities|Enum|Equal(Enum) _curentvalue "NewEnumerator10") (Math|Rotator|GetRotationXVector (Math|Rotator|MakeRotator (.roll (Transformation|GetActorRotation _currentbaractor)) (.pitch (Transformation|GetActorRotation _currentbaractor)) (select (> (Math|Vector|DotProduct (Transformation|GetActorForwardVector _currentbaractor) (Transformation|GetActorForwardVector (Variables|Default|GetcharRef))) 0.0) (.yaw (Transformation|GetActorRotation _currentbaractor)) (- (.yaw (Transformation|GetActorRotation _currentbaractor)) 1.8e+02)))) (Math|Rotator|GetRotationXVector (Math|Rotator|MakeRotator (.Roll (Math|Rotator|BreakRotator (Transformation|GetActorRotation _currentbaractor))) (.Pitch (Math|Rotator|BreakRotator (Transformation|GetActorRotation _currentbaractor))) (Math|Float|SelectFloat (.Yaw (Math|Rotator|BreakRotator (Transformation|GetActorRotation _currentbaractor))) (+ (.Yaw (Math|Rotator|BreakRotator (Transformation|GetActorRotation _currentbaractor))) 1.8e+02) (> (Math|Vector|DotProduct (Transformation|GetActorForwardVector _currentbaractor) (Transformation|GetActorForwardVector (Variables|Default|GetcharRef))) 0.0))))) false 0.0)
      (Default|AdjustPosition _charref_4 (Transformation|GetActorLocation _charref_4) (- (+ (* (* (Transformation|GetActorForwardVector _currentbaractor) (Math|Float|SelectFloat (* (Math|Float|Sign(Float) (Math|Vector|DotProduct (Math|Vector|Normalize (Math|Vector|MakeVector (.x (- (Transformation|GetActorLocation _currentbaractor) _returnvalue)) (.y (- (Transformation|GetActorLocation _currentbaractor) _returnvalue)) 0.0)) (Transformation|GetActorForwardVector _currentbaractor))) -1.0) (* (Math|Float|Sign(Float) (Math|Vector|DotProduct (Transformation|GetActorForwardVector _currentbaractor) (Transformation|GetActorForwardVector _charref_3))) -1.0) (Utilities|Enum|Equal(Enum) _curentvalue "NewEnumerator10"))) (Math|Vector|VectorLength (Math|Vector|MakeVector (.x (- (Transformation|GetActorLocation _currentbaractor) _returnvalue)) (.y (- (Transformation|GetActorLocation _currentbaractor) _returnvalue)) 0.0))) (Transformation|GetActorLocation _currentbaractor) (Math|Vector|SelectVector "0, 0, 0" (Math|Vector|SelectVector (* (Math|Vector|Normalize (Transformation|GetActorForwardVector _charref_2)) 5e+01) "0, 0, 0" (> (Math|Vector|VectorLength (Pawn|Components|CharacterMovement|GetLastUpdateVelocity (Variables|/Script/Engine.Character|GetCharacterMovement _charref_2))) 0.0)) (Utilities|Enum|Equal(Enum) _curentvalue "NewEnumerator10"))) _returnvalue) false true true))
    (:Is%20Not%20Valid
      (Development|PrintString 0 "INVALID BAR" true true "(R=1.000000,G=0.000000,B=0.071486,A=1.000000)")
      (return))))

(fn InputMoveForward
  (params (inputVal :type Float%20%28single-precision%29))
  (bind _charref (Variables|Default|GetcharRef))
  (|CallParentFunction 0.0)
  (bind _output_get (Variables|/Game/AmplifyAnimationPack/Blueprints/Character/BP_Character.BP_Character_C|SetInputForward _charref inputVal))
  (Default|SetInputFwdVal (Variables|/Game/AmplifyAnimationPack/Blueprints/Character/BP_Character.BP_Character_C|GetcharAnimCommunicator _charref) _output_get))

(fn UpdateStateAnimation
  (bind _charref (Variables|Default|GetcharRef))
  (bind _charref_2 (Variables|Default|GetCharRef))
  (bind _charanimcommunicator (Variables|/Game/AmplifyAnimationPack/Blueprints/Character/BP_Character.BP_Character_C|GetcharAnimCommunicator _charref))
  (bind _charanimcommunicator_2 (Variables|/Game/AmplifyAnimationPack/Blueprints/Character/BP_Character.BP_Character_C|GetcharAnimCommunicator _charref_2))
  (|CallParentFunction)
  (Utilities|IsValid (Utilities|ToObject(Interface) _charanimcommunicator)
    (:Is%20Valid
      (bind _curentvalue (Default|GetBarWalkActionVal _charanimcommunicator))
      (if (Utilities|Enum|NotEqual(Enum) _curentvalue "NewEnumerator10")
        (bind _newdirection (Default|UpdateDirection _charref_2 false))
        (Default|SetDirectionVal _charanimcommunicator_2 _newdirection)
        (bind _curentvalue_2 (Default|GetInputRightVal _charanimcommunicator_2))
        (bind _curentvalue_3 (Default|GetInputFwdVal _charanimcommunicator_2))
        (Default|SetSpeedVal _charanimcommunicator_2 (Math|Float|Clamp(Float) (+ (Math|Float|Absolute(Float) _curentvalue_3) (Math|Float|Absolute(Float) _curentvalue_2))))
        (else
          (return))))
    (:Is%20Not%20Valid
      (return))))

(fn InputMoveRight
  (params (inputVal :type Float%20%28single-precision%29))
  (bind _charref (Variables|Default|GetcharRef))
  (|CallParentFunction 0.0)
  (bind _output_get (Variables|/Game/AmplifyAnimationPack/Blueprints/Character/BP_Character.BP_Character_C|SetInputRight _charref inputVal))
  (Default|SetInputRightVal (Variables|/Game/AmplifyAnimationPack/Blueprints/Character/BP_Character.BP_Character_C|GetcharAnimCommunicator _charref) _output_get))

(fn UpdateState
  (params (deltaTime :type Float%20%28single-precision%29))
  (bind _charref (Variables|Default|GetcharRef))
  (|CallParentFunction 0.0)
  (bind _curentvalue (Default|GetBarWalkActionVal (Variables|/Game/AmplifyAnimationPack/Blueprints/Character/BP_Character.BP_Character_C|GetcharAnimCommunicator (Variables|Default|GetcharRef))))
  (if (Utilities|Enum|NotEqual(Enum) _curentvalue "NewEnumerator10")
    (bind (_groundhitresult _isgrounded) (Default|GroundSpheretraceDetector _charref))
    (if _isgrounded
      (if (!= (Utilities|GetClass (.HitActor (Collision|BreakHitResult _groundhitresult))) "/Game/AmplifyAnimationPack/Blueprints/Interactables/BP_BarActor.BP_BarActor_C")
        (Default|ChangeCurrentState (Variables|Default|GetcharRef) "/Game/AmplifyAnimationPack/Blueprints/Character/CharacterStates/BP_GroundedState.BP_GroundedState_C"))
      (else
        (Default|ChangeCurrentState _charref "/Game/AmplifyAnimationPack/Blueprints/Character/CharacterStates/BP_FallingState.BP_FallingState_C")))
    (else
      (return))))

(fn CheckIsonBar
  (bind _groundhitresult (Default|GroundSpheretraceDetector (Variables|Default|GetcharRef)))
  (if (== (Utilities|GetClass (.HitActor (Collision|BreakHitResult _groundhitresult))) "/Game/AmplifyAnimationPack/Blueprints/Interactables/BP_BarActor.BP_BarActor_C")
    (bind _asbp_bar_actor (Utilities|Casting|CastToBP_BarActor (.HitActor (Collision|BreakHitResult _groundhitresult))))
    (return _asbp_bar_actor)
    (else
      (return 0))))

(fn OrienttoBar
  (bind _currentbaractor (CallFunction|CheckIsonBar))
  (Default|AdjustRotation (Variables|Default|GetcharRef) (* (Transformation|GetActorForwardVector _currentbaractor) (Math|Float|Sign(Float) (Math|Vector|DotProduct (Transformation|GetActorForwardVector _currentbaractor) (Transformation|GetActorForwardVector (Variables|Default|GetcharRef))))) false 0.0))

(fn InputInteract
  (|CallParentFunction)
  (if (Variables|Default|GetcanDrop)
    (Default|SetBarWalkActionVal (Variables|/Game/AmplifyAnimationPack/Blueprints/Character/BP_Character.BP_Character_C|GetcharAnimCommunicator (Variables|Default|GetcharRef)) "NewEnumerator10")))