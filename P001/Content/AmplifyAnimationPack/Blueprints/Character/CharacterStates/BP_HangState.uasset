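; Character state for hanging on ledges, which puts movement in Flying mode with a narrowed capsule and slows input to trace-validated actions.
; Move inputs run CharRef climb traces to pick shimmy, corner or jump-ready hang actions, written to CharAnimCommunicator for animation.
; Jump triggers jumps or releases the plane constraint to climb, and crouch-hold readies a back jump.
; Interact can switch to BP_HangClimbState, while attack derives its direction from input.
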(fn EnterState
  (params (prevStateClass :type BP%20Character%20State%20Base%20Class%20Reference))
  (bind _charref (Variables|Default|GetcharRef))
  (bind _charref_2 (Variables|Default|GetcharRef))
  (bind _charactermovement (Variables|/Script/Engine.Character|GetCharacterMovement _charref))
  (bind _charanimcommunicator (Variables|/Game/AmplifyAnimationPack/Blueprints/Character/BP_Character.BP_Character_C|GetcharAnimCommunicator _charref_2))
  (|CallParentFunction 0)
  (Variables|/Script/Engine.SpringArmComponent|SetCameraLagSpeed (Variables|/Game/AmplifyAnimationPack/Blueprints/Character/BP_Character.BP_Character_C|GetCameraArm _charref) (Variables|/Game/AmplifyAnimationPack/Blueprints/Character/BP_Character.BP_Character_C|GetcameraLagSpeedHang _charref))
  (Default|SetNewCapsuleRadius _charref 2e+01 0.0)
  (Pawn|Components|CharacterMovement|SetMovementMode _charactermovement "MOVE_Flying" 0)
  (Class|MovementComponent|SetPlaneConstraintAxisSetting _charactermovement "Z")
  (Default|SetMovementStateVal _charanimcommunicator "NewEnumerator10")
  (Default|SetSpeedVal _charanimcommunicator 0.0)
  (Default|SetHangActionVal _charanimcommunicator "NewEnumerator0")
  (Variables|Default|SetcanMove false))

(fn InputMoveForward
  (params (inputVal :type Float%20%28single-precision%29))
  (bind _charref (Variables|Default|GetcharRef))
  (bind _charref_2 (Variables|Default|GetcharRef))
  (bind _charref_3 (Variables|Default|GetcharRef))
  (bind _charanimcommunicator (Variables|/Game/AmplifyAnimationPack/Blueprints/Character/BP_Character.BP_Character_C|GetcharAnimCommunicator _charref_2))
  (bind _charanimcommunicator_2 (Variables|/Game/AmplifyAnimationPack/Blueprints/Character/BP_Character.BP_Character_C|GetcharAnimCommunicator _charref_3))
  (bind _charanimcommunicator_3 (Variables|/Game/AmplifyAnimationPack/Blueprints/Character/BP_Character.BP_Character_C|GetcharAnimCommunicator _charref))
  (|CallParentFunction 0.0)
  (bind _output_get (Variables|/Game/AmplifyAnimationPack/Blueprints/Character/BP_Character.BP_Character_C|SetInputForward _charref inputVal))
  (bind _currentval (Default|SetInputFwdVal _charanimcommunicator_3 _output_get))
  (if (!= _currentval 0.0)
    (bind _curentvalue (Default|GetHangActionVal _charanimcommunicator_3))
    (if (not (or (not (Variables|Default|GetcanMove)) (Utilities|Enum|Equal(Enum) _curentvalue "NewEnumerator1")))
      (bind _curentvalue_2 (Default|GetInputRightVal _charanimcommunicator_3))
      (bind _ishitting (Default|ClimbSpheretraceHangJump (Variables|Default|GetcharRef) _curentvalue_2 inputVal))
      (if _ishitting
        (Default|SetHangActionVal _charanimcommunicator_2 "NewEnumerator4")
        (Components|Movement|StopMovementImmediately (Variables|/Script/Engine.Character|GetCharacterMovement _charref_2))
        (bind _curentvalue_3 (Default|GetInputRightVal _charanimcommunicator))
        (Default|SetHangReachArmVal _charanimcommunicator (select (>= _curentvalue_3 0.0) "NewEnumerator1" "NewEnumerator0"))
        (else
          (Default|SetHangActionVal _charanimcommunicator_2 "NewEnumerator0"))))))

(fn InputMoveRight
  (params (inputVal :type Float%20%28single-precision%29))
  (bind _charref (Variables|Default|GetcharRef))
  (bind _charref_2 (Variables|Default|GetcharRef))
  (bind _charref_3 (Variables|Default|GetcharRef))
  (bind _charref_4 (Variables|Default|GetcharRef))
  (bind _charref_5 (Variables|Default|GetcharRef))
  (bind _charanimcommunicator (Variables|/Game/AmplifyAnimationPack/Blueprints/Character/BP_Character.BP_Character_C|GetcharAnimCommunicator _charref_5))
  (bind _charanimcommunicator_2 (Variables|/Game/AmplifyAnimationPack/Blueprints/Character/BP_Character.BP_Character_C|GetcharAnimCommunicator _charref_3))
  (|CallParentFunction 0.0)
  (if (Variables|Default|GetcanMove)
    (bind _output_get (Variables|/Game/AmplifyAnimationPack/Blueprints/Character/BP_Character.BP_Character_C|SetInputRight _charref inputVal))
    (bind _currentval (Default|SetInputRightVal (Variables|/Game/AmplifyAnimationPack/Blueprints/Character/BP_Character.BP_Character_C|GetcharAnimCommunicator _charref) _output_get))
    (if (!= _currentval 0.0)
      (Variables|Default|SetmovementDirection _currentval)
      (bind _ishitting (Default|ClimbSpheretraceHangMovement (Variables|Default|GetcharRef) inputVal))
      (if _ishitting
        (bind _ishitting_2 (Default|ClimbSpheretraceHangCorner (Variables|Default|GetcharRef) inputVal -1.0 7e+01))
        (if _ishitting_2
          (Default|SetHangActionVal _charanimcommunicator "NewEnumerator5")
          (else
            (Default|SetHangActionVal _charanimcommunicator "NewEnumerator3")
            (Default|SetHangAttackDirVal _charanimcommunicator (select (> inputVal 0.0) "NewEnumerator12" "NewEnumerator13"))))
        (else
          (bind _curentvalue (Default|GetInputFwdVal (Variables|/Game/AmplifyAnimationPack/Blueprints/Character/BP_Character.BP_Character_C|GetcharAnimCommunicator (Variables|Default|GetcharRef))))
          (bind _ishitting_3 (Default|ClimbSpheretraceHangJump _charref_2 inputVal _curentvalue))
          (if _ishitting_3
            (bind _curentvalue_2 (Default|GetHangActionVal (Variables|/Game/AmplifyAnimationPack/Blueprints/Character/BP_Character.BP_Character_C|GetcharAnimCommunicator _charref_2)))
            (if (Utilities|Enum|NotEqual(Enum) _curentvalue_2 "NewEnumerator1")
              (Default|SetHangActionVal (Variables|/Game/AmplifyAnimationPack/Blueprints/Character/BP_Character.BP_Character_C|GetcharAnimCommunicator _charref_4) "NewEnumerator4")
              (Components|Movement|StopMovementImmediately (Variables|/Script/Engine.Character|GetCharacterMovement _charref_4)))
            (else
              (bind _ishitting_4 (Default|ClimbSpheretraceHangCorner _charref_3 inputVal 1.0 4e+01))
              (if _ishitting_4
                (Default|SetHangActionVal _charanimcommunicator_2 "NewEnumerator2")
                (else
                  (bind _ishitting_5 (Default|ClimbSpheretraceHangCorner (Variables|Default|GetcharRef) inputVal -1.0 4e+01))
                  (if _ishitting_5
                    (Default|SetHangActionVal _charanimcommunicator_2 "NewEnumerator5")
                    (else
                      (Default|SetHangActionVal _charanimcommunicator_2 "NewEnumerator0"))))))))))
    (else
      (return))))

(fn InputJump
  (bind _charref (Variables|Default|GetcharRef))
  (bind _charref_2 (Variables|Default|GetcharRef))
  (bind _charref_3 (Variables|Default|GetcharRef))
  (bind _charref_4 (Variables|Default|GetcharRef))
  (bind _charanimcommunicator (Variables|/Game/AmplifyAnimationPack/Blueprints/Character/BP_Character.BP_Character_C|GetcharAnimCommunicator _charref))
  (bind _charanimcommunicator_2 (Variables|/Game/AmplifyAnimationPack/Blueprints/Character/BP_Character.BP_Character_C|GetcharAnimCommunicator _charref_3))
  (bind _charanimcommunicator_3 (Variables|/Game/AmplifyAnimationPack/Blueprints/Character/BP_Character.BP_Character_C|GetcharAnimCommunicator _charref_2))
  (|CallParentFunction)
  (bind _curentvalue (Default|GetInputRightVal _charanimcommunicator_3))
  (bind _curentvalue_2 (Default|GetInputFwdVal _charanimcommunicator_3))
  (if (or (!= _curentvalue 0.0) (!= _curentvalue_2 0.0))
    (bind _curentvalue_3 (Default|GetHangActionVal _charanimcommunicator_2))
    (if (or (Utilities|Enum|Equal(Enum) _curentvalue_3 "NewEnumerator4") (Utilities|Enum|Equal(Enum) _curentvalue_3 "NewEnumerator8"))
      (Default|SetHangActionVal _charanimcommunicator "NewEnumerator1" :!label _label)
      (Variables|Default|SetcanMove false :!label _label_2))
    (else
      (bind _curentvalue_4 (Default|GetHangActionVal _charanimcommunicator_2))
      (if (Utilities|Enum|Equal(Enum) _curentvalue_4 "NewEnumerator8")
        (goto _label)
        (else
          (Class|MovementComponent|SetPlaneConstraintEnabled (Variables|/Script/Engine.Character|GetCharacterMovement _charref_3) false)
          (Default|SetIsHangClimbingVal _charanimcommunicator true)
          (Default|SetHangActionVal _charanimcommunicator "NewEnumerator6")
          (Variables|/Script/Engine.SpringArmComponent|SetCameraLagSpeed (Variables|/Game/AmplifyAnimationPack/Blueprints/Character/BP_Character.BP_Character_C|GetCameraArm _charref_4) (Variables|/Game/AmplifyAnimationPack/Blueprints/Character/BP_Character.BP_Character_C|GetcameraLagSpeedHeightFactor _charref_4))
          (goto _label_2))))))

(fn ExitState
  (|CallParentFunction)
  (Class|MovementComponent|SetPlaneConstraintEnabled (Variables|/Script/Engine.Character|GetCharacterMovement (Variables|Default|GetcharRef)) false))

(fn InputInteract
  (bind _charref (Variables|Default|GetcharRef))
  (|CallParentFunction)
  (if (Variables|Default|GetcanMove)
    (bind _ishitting (Default|ClimbSpheretraceHangClimb _charref))
    (if (not _ishitting)
      (Default|ChangeCurrentState _charref "/Game/AmplifyAnimationPack/Blueprints/Character/CharacterStates/BP_HangClimbState.BP_HangClimbState_C")
      (Default|SetIsHangClimbingVal (Variables|/Game/AmplifyAnimationPack/Blueprints/Character/BP_Character.BP_Character_C|GetcharAnimCommunicator _charref) true)
      (else
        (return)))
    (else
      (return))))

(fn InputAttack
  (params (AttackState :type Character_CombatAction_Enum%20Enum :default "NewEnumerator0"))
  (bind _charref (Variables|Default|GetcharRef))
  (bind _charanimcommunicator (Variables|/Game/AmplifyAnimationPack/Blueprints/Character/BP_Character.BP_Character_C|GetcharAnimCommunicator _charref))
  (|CallParentFunction "NewEnumerator0")
  (bind _curentvalue (Default|GetHangAttackDirVal _charanimcommunicator))
  (bind _curentvalue_2 (Default|GetInputRightVal _charanimcommunicator))
  (bind _curentvalue_3 (Default|GetInputFwdVal _charanimcommunicator))
  (bind _finalattackdir (CallFunction|SetHangAttackDir _curentvalue _curentvalue_2 _curentvalue_3))
  (Default|SetHangAttackDirVal _charanimcommunicator _finalattackdir)
  (Default|AttackStart _charref AttackState))

(fn InputCrouchHold
  (params (inputVal :type Float%20%28single-precision%29))
  (bind _charref (Variables|Default|GetcharRef))
  (bind _charref_2 (Variables|Default|GetcharRef))
  (bind _charanimcommunicator (Variables|/Game/AmplifyAnimationPack/Blueprints/Character/BP_Character.BP_Character_C|GetcharAnimCommunicator _charref))
  (bind _charanimcommunicator_2 (Variables|/Game/AmplifyAnimationPack/Blueprints/Character/BP_Character.BP_Character_C|GetcharAnimCommunicator _charref_2))
  (|CallParentFunction 0.0)
  (if (!= inputVal 0.0)
    (bind _curentvalue (Default|GetHangActionVal _charanimcommunicator_2))
    (if (Utilities|Enum|Equal(Enum) _curentvalue "NewEnumerator0")
      (bind _ishitting (Default|ClimbLinetraceHangJumpBack (Variables|Default|GetcharRef) 0.0))
      (if _ishitting
        (Default|SetHangActionVal _charanimcommunicator "NewEnumerator8")))
    (else
      (bind _curentvalue_2 (Default|GetHangActionVal _charanimcommunicator_2))
      (if (Utilities|Enum|Equal(Enum) _curentvalue_2 "NewEnumerator8")
        (Default|SetHangActionVal _charanimcommunicator "NewEnumerator0")))))

(fn UpdateState
  (params (deltaTime :type Float%20%28single-precision%29))
  (|CallParentFunction 0.0)
  (bind _curentvalue (Default|GetHangActionVal (Variables|/Game/AmplifyAnimationPack/Blueprints/Character/BP_Character.BP_Character_C|GetcharAnimCommunicator (Variables|Default|GetcharRef))))
  (if (Utilities|Enum|Equal(Enum) _curentvalue "NewEnumerator3")
    (bind _ishitting (Default|ClimbSpheretraceHangMovement (Variables|Default|GetcharRef) (Variables|Default|GetmovementDirection)))
    (if (not _ishitting)
      (Default|SetHangActionVal (Variables|/Game/AmplifyAnimationPack/Blueprints/Character/BP_Character.BP_Character_C|GetcharAnimCommunicator (Variables|Default|GetcharRef)) "NewEnumerator0"))))

(fn SetHangAttackDir
  (params (initialAttackDir :type Character_HangAttackDirections_Enum%20Enum :default "NewEnumerator9") (inputRight :type Float%20%28single-precision%29) (inputForward :type Float%20%28single-precision%29))
  (bind _returnvalue (!= inputRight 0.0))
  (bind _returnvalue_2 (> inputRight 0.0))
  (if (and (== inputRight 0.0) (== inputForward 0.0))
    (return initialAttackDir)
    (elif (> inputForward 0.0)
      (if _returnvalue
        (return (select _returnvalue_2 "NewEnumerator10" "NewEnumerator11"))
        (else
          (return "NewEnumerator9")))
      (elif (< inputForward 0.0)
        (if _returnvalue
          (return (select _returnvalue_2 "NewEnumerator15" "NewEnumerator16"))
          (else
            (return "NewEnumerator14")))
        (else
          (return (select _returnvalue_2 "NewEnumerator12" "NewEnumerator13")))))))