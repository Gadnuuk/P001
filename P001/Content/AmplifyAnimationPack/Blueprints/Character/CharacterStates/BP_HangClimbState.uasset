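; Character state for hang climbing in the Amplify Animation Pack's character state system.
; On entry it sets the movement state on the anim communicator, disables capsule collision and camera arm collision tests, switches movement to Flying and resets camera lag speed to default.
; On exit it restores capsule collision, camera collision testing and Walking movement.
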(fn EnterState
  (params (prevStateClass :type BP%20Character%20State%20Base%20Class%20Reference))
  (bind _charref (Variables|Default|GetcharRef))
  (bind _charref_2 (Variables|Default|GetCharRef))
  (bind _charref_3 (Variables|Default|GetcharRef))
  (|CallParentFunction 0)
  (Variables|/Script/Engine.SpringArmComponent|SetbDoCollisionTest (Variables|/Game/AmplifyAnimationPack/Blueprints/Character/BP_Character.BP_Character_C|GetCameraArm _charref) false)
  (Default|SetMovementStateVal (Variables|/Game/AmplifyAnimationPack/Blueprints/Character/BP_Character.BP_Character_C|GetcharAnimCommunicator _charref) "NewEnumerator11")
  (Collision|SetCollisionEnabled (Variables|/Script/Engine.Character|GetCapsuleComponent _charref_2) "NoCollision")
  (Pawn|Components|CharacterMovement|SetMovementMode (Variables|/Script/Engine.Character|GetCharacterMovement _charref_2) "MOVE_Flying" 0)
  (Variables|/Script/Engine.SpringArmComponent|SetCameraLagSpeed (Variables|/Game/AmplifyAnimationPack/Blueprints/Character/BP_Character.BP_Character_C|GetCameraArm _charref_3) (Variables|/Game/AmplifyAnimationPack/Blueprints/Character/BP_Character.BP_Character_C|GetcameraLagSpeedDefault _charref_3)))

(fn ExitState
  (bind _charref (Variables|Default|GetcharRef))
  (|CallParentFunction)
  (Variables|/Script/Engine.SpringArmComponent|SetbDoCollisionTest (Variables|/Game/AmplifyAnimationPack/Blueprints/Character/BP_Character.BP_Character_C|GetCameraArm _charref) true)
  (Pawn|Components|CharacterMovement|SetMovementMode (Variables|/Script/Engine.Character|GetCharacterMovement _charref) "MOVE_Walking" 0)
  (Collision|SetCollisionEnabled (Variables|/Script/Engine.Character|GetCapsuleComponent (Variables|Default|GetcharRef)) "QueryAndPhysics"))