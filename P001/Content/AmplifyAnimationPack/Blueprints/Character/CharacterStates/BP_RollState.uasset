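; Roll state for the Amplify Animation Pack character's state machine.
; On enter, it reverses the crouch adjustment for one specific prior movement state, then sets a new movement state and clears the can-fall-off-roll flag through CharAnimCommunicator.
; Each update runs a ground sphere trace and switches to BP_FallingState if the character is ungrounded while that flag is set.
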(fn EnterState
  (params (prevStateClass :type BP%20Character%20State%20Base%20Class%20Reference))
  (bind _charref (Variables|Default|GetcharRef))
  (bind _charref_2 (Variables|Default|GetcharRef))
  (bind _charanimcommunicator (Variables|/Game/AmplifyAnimationPack/Blueprints/Character/BP_Character.BP_Character_C|GetcharAnimCommunicator _charref))
  (|CallParentFunction 0)
  (bind _curentvalue (Default|GetMovementStateVal (Variables|/Game/AmplifyAnimationPack/Blueprints/Character/BP_Character.BP_Character_C|GetcharAnimCommunicator (Variables|Default|GetcharRef))))
  (if (Utilities|Enum|Equal(Enum) _curentvalue "NewEnumerator2")
    (Default|CrouchAdjustCharacter _charref_2 false (Transformation|GetActorLocation _charref_2)))
  (Default|SetMovementStateVal _charanimcommunicator "NewEnumerator16")
  (Default|SetCanFallOfRollVal _charanimcommunicator false))

(fn UpdateState
  (params (deltaTime :type Float%20%28single-precision%29))
  (bind _charref (Variables|Default|GetcharRef))
  (|CallParentFunction 0.0)
  (bind _isgrounded (Default|GroundSpheretraceDetector _charref))
  (bind _curentvalue (Default|GetCanFallOfRollVal (Variables|/Game/AmplifyAnimationPack/Blueprints/Character/BP_Character.BP_Character_C|GetcharAnimCommunicator _charref)))
  (if (and _curentvalue (not _isgrounded))
    (Default|ChangeCurrentState _charref "/Game/AmplifyAnimationPack/Blueprints/Character/CharacterStates/BP_FallingState.BP_FallingState_C")))