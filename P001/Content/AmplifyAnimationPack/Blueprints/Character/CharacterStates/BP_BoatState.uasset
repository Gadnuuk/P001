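; Character state for boarding, steering and leaving kayak, sail, row, motor and gondola boats.
; On entry it snaps the character to a swim or grounded entry point, switches to flying without collision and blends to the boat camera.
; Input adds force and yaw to the boat, scaled by animation curves for all but sail and motor types.
; Exiting uses a linetrace to pick the animation, with per-type camera blends back to the character.
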(fn EnterState
  (params (prevStateClass :type BP%20Character%20State%20Base%20Class%20Reference))
  (bind _charref (Variables|Default|GetcharRef))
  (bind _returnvalue (Transformation|GetActorLocation _charref))
  (bind _charanimcommunicator (Variables|/Game/AmplifyAnimationPack/Blueprints/Character/BP_Character.BP_Character_C|GetcharAnimCommunicator _charref))
  (|CallParentFunction 0)
  (bind _asbp_boat_actor (Utilities|Casting|CastToBP_BoatActor (Variables|/Game/AmplifyAnimationPack/Blueprints/Character/BP_Character.BP_Character_C|GetobjectToInteract (Variables|Default|GetcharRef))))
  (bind _output_get (Variables|Default|SetcurrentBoatActor _asbp_boat_actor))
  (CallFunction|AssingBoatType _output_get)
  (Default|CharacterEntered _output_get)
  (bind _curentvalue (Default|GetMovementStateVal (Variables|/Game/AmplifyAnimationPack/Blueprints/Character/BP_Character.BP_Character_C|GetcharAnimCommunicator _charref)))
  (Collision|SetCollisionEnabled (Variables|/Script/Engine.Character|GetCapsuleComponent _charref) "NoCollision")
  (Pawn|Components|CharacterMovement|SetMovementMode (Variables|/Script/Engine.Character|GetCharacterMovement _charref) "MOVE_Flying" 0)
  (Default|ChangeCamera _charref (Variables|Default|GetcurrentBoatActor) 2.0)
  (Default|AdjustPosition _charref _returnvalue (- (Transformation|GetWorldLocation (select (Utilities|Enum|Equal(Enum) _curentvalue "NewEnumerator26") (Variables|/Game/AmplifyAnimationPack/Blueprints/Interactables/Boat/BP_BoatActor.BP_BoatActor_C|GetEnterPoint_Swim (Variables|Default|GetcurrentBoatActor)) (Variables|/Game/AmplifyAnimationPack/Blueprints/Interactables/Boat/BP_BoatActor.BP_BoatActor_C|GetEnterPoint_Grounded (Variables|Default|GetcurrentBoatActor)))) _returnvalue) false true (not (Utilities|Enum|Equal(Enum) _curentvalue "NewEnumerator26")))
  (Default|AdjustRotation _charref (Math|Rotator|GetRotationXVector (Transformation|GetWorldRotation (select (Utilities|Enum|Equal(Enum) _curentvalue "NewEnumerator26") (Variables|/Game/AmplifyAnimationPack/Blueprints/Interactables/Boat/BP_BoatActor.BP_BoatActor_C|GetEnterPoint_Swim (Variables|Default|GetcurrentBoatActor)) (Variables|/Game/AmplifyAnimationPack/Blueprints/Interactables/Boat/BP_BoatActor.BP_BoatActor_C|GetEnterPoint_Grounded (Variables|Default|GetcurrentBoatActor))))) true 2e+01)
  (bind _curentvalue_2 (Default|GetMovementStateVal _charanimcommunicator))
  (Default|SetSpeedVal _charanimcommunicator 0.0)
  (bind _currentvalue (Default|SetBoatActionVal _charanimcommunicator (select (Utilities|Enum|Equal(Enum) _curentvalue_2 "NewEnumerator26") "NewEnumerator1" "NewEnumerator0")))
  (Default|SetMovementStateVal _charanimcommunicator "NewEnumerator27")
  (Variables|Default|SetcanMove false)
  (if (Utilities|Enum|Equal(Enum) _currentvalue "NewEnumerator0")
    (Transformation|AttachActorToActor (Variables|Default|GetcharRef) (Variables|Default|GetcurrentBoatActor) "None" "KeepWorld" "KeepWorld" "KeepWorld" false)))

(fn InputMoveForward
  (params (inputVal :type Float%20%28single-precision%29))
  (bind _currentboatactor (Variables|Default|GetcurrentBoatActor))
  (bind _currentboatactor_2 (Variables|Default|GetcurrentBoatActor))
  (bind _charref (Variables|Default|GetcharRef))
  (bind _accelspeed (Variables|/Game/AmplifyAnimationPack/Blueprints/Interactables/Boat/BP_BoatActor.BP_BoatActor_C|GetaccelSpeed _currentboatactor))
  (bind _charanimcommunicator (Variables|/Game/AmplifyAnimationPack/Blueprints/Character/BP_Character.BP_Character_C|GetcharAnimCommunicator _charref))
  (|CallParentFunction 0.0)
  (bind _output_get (Variables|/Game/AmplifyAnimationPack/Blueprints/Character/BP_Character.BP_Character_C|SetInputForward _charref inputVal))
  (bind _currentval (Default|SetInputFwdVal _charanimcommunicator _output_get))
  (bind _curentvalue (Default|GetBoatTypeVal _charanimcommunicator))
  (bind _asanim_instance (Utilities|Casting|CastToAnimInstance _charanimcommunicator))
  (Physics|AddForce (Variables|/Game/AmplifyAnimationPack/Blueprints/Interactables/Boat/BP_BoatActor.BP_BoatActor_C|GetMesh _currentboatactor) (Math|Vector|MakeVector (.x (* (* (Transformation|GetActorForwardVector _currentboatactor_2) (Math|Float|SelectFloat (Math|Float|SelectFloat _accelspeed (* _accelspeed (Animation|Curves|GetCurveValue _asanim_instance "Boat_MovementAmount") (Math|Float|Absolute(Float) _currentval)) (or (Utilities|Enum|Equal(Enum) _curentvalue "NewEnumerator1") (Utilities|Enum|Equal(Enum) _curentvalue "NewEnumerator3"))) 0.0 (and (< (Math|Vector|VectorLength (Transformation|GetVelocity _currentboatactor_2)) (Variables|/Game/AmplifyAnimationPack/Blueprints/Interactables/Boat/BP_BoatActor.BP_BoatActor_C|GetmaxSpeed _currentboatactor_2)) (Variables|Default|GetcanMove)))) _currentval)) (.y (* (* (Transformation|GetActorForwardVector _currentboatactor_2) (Math|Float|SelectFloat (Math|Float|SelectFloat _accelspeed (* _accelspeed (Animation|Curves|GetCurveValue _asanim_instance "Boat_MovementAmount") (Math|Float|Absolute(Float) _currentval)) (or (Utilities|Enum|Equal(Enum) _curentvalue "NewEnumerator1") (Utilities|Enum|Equal(Enum) _curentvalue "NewEnumerator3"))) 0.0 (and (< (Math|Vector|VectorLength (Transformation|GetVelocity _currentboatactor_2)) (Variables|/Game/AmplifyAnimationPack/Blueprints/Interactables/Boat/BP_BoatActor.BP_BoatActor_C|GetmaxSpeed _currentboatactor_2)) (Variables|Default|GetcanMove)))) _currentval)) 0.0) "None" true))

(fn ExitState
  (|CallParentFunction)
  (Default|CharacterLeft (Variables|Default|GetcurrentBoatActor)))

(fn InputMoveRight
  (params (inputVal :type Float%20%28single-precision%29))
  (bind _currentboatactor (Variables|Default|GetcurrentBoatActor))
  (bind _charref (Variables|Default|GetcharRef))
  (bind _currentboatactor_2 (Variables|Default|GetcurrentBoatActor))
  (bind _returnvalue (Transformation|GetActorRotation _currentboatactor_2))
  (bind _charanimcommunicator (Variables|/Game/AmplifyAnimationPack/Blueprints/Character/BP_Character.BP_Character_C|GetcharAnimCommunicator _charref))
  (|CallParentFunction 0.0)
  (bind _output_get (Variables|/Game/AmplifyAnimationPack/Blueprints/Character/BP_Character.BP_Character_C|SetInputRight _charref inputVal))
  (bind _currentval (Default|SetInputRightVal _charanimcommunicator _output_get))
  (bind _asanim_instance (Utilities|Casting|CastToAnimInstance _charanimcommunicator))
  (bind _curentvalue (Default|GetBoatTypeVal _charanimcommunicator))
  (bind _deltaseconds (Default|GetDeltaTime (Variables|Default|GetcharRef)))
  (Transformation|SetActorRotation _currentboatactor_2 (Math|Rotator|MakeRotator (.roll _returnvalue) (.pitch _returnvalue) (Math|Float|SelectFloat (.yaw (Math|Conversions|RotationFromXVector (Math|Interpolation|VInterptoConstant (Transformation|GetActorForwardVector _currentboatactor) (* (Transformation|GetActorRightVector _currentboatactor) (Math|Float|SelectFloat _currentval (* _currentval (Animation|Curves|GetCurveValue _asanim_instance "Boat_RotationAmount")) (or (Utilities|Enum|Equal(Enum) _curentvalue "NewEnumerator1") (Utilities|Enum|Equal(Enum) _curentvalue "NewEnumerator3")))) _deltaseconds (Variables|/Game/AmplifyAnimationPack/Blueprints/Interactables/Boat/BP_BoatActor.BP_BoatActor_C|GetrotationSpeed _currentboatactor_2)))) (.yaw _returnvalue) (Variables|Default|GetcanMove)))))

(fn InputInteract
  (|CallParentFunction)
  (if (Variables|Default|GetcanMove)
    (Default|PrepareforCharGettingOut (Variables|Default|GetcurrentBoatActor))))

(fn AssingBoatType
  (params (currBoatActor :type BP%20Boat%20Actor%20Object%20Reference))
  (bind _returnvalue (Utilities|GetClass currBoatActor))
  (Default|SetBoatTypeVal (Variables|/Game/AmplifyAnimationPack/Blueprints/Character/BP_Character.BP_Character_C|GetcharAnimCommunicator (Variables|Default|GetcharRef)) (select (== _returnvalue "/Game/AmplifyAnimationPack/Blueprints/Interactables/Boat/BP_KayakBoatActor.BP_KayakBoatActor_C") "NewEnumerator2" (select (== _returnvalue "/Game/AmplifyAnimationPack/Blueprints/Interactables/Boat/BP_SailBoatActor.BP_SailBoatActor_C") "NewEnumerator1" (select (== _returnvalue "/Game/AmplifyAnimationPack/Blueprints/Interactables/Boat/BP_RowBoatActor.BP_RowBoatActor_C") "NewEnumerator4" (select (== _returnvalue "/Game/AmplifyAnimationPack/Blueprints/Interactables/Boat/BP_MotorBoatActor.BP_MotorBoatActor_C") "NewEnumerator3" "NewEnumerator0"))))))

(fn GetOutOfBoat
  (bind _charref (Variables|Default|GetcharRef))
  (bind _charref_2 (Variables|Default|GetcharRef))
  (bind _charanimcommunicator (Variables|/Game/AmplifyAnimationPack/Blueprints/Character/BP_Character.BP_Character_C|GetcharAnimCommunicator _charref))
  (if (Variables|Default|GetcanMove)
    (Variables|Default|SetcanMove false)
    (bind _cangetout (Default|BoatGetOutLinetrace _charref))
    (bind _currentvalue (Default|SetBoatActionVal _charanimcommunicator (select _cangetout "NewEnumerator3" "NewEnumerator4")))
    (bind _curentvalue (Default|GetBoatTypeVal _charanimcommunicator))
    (Default|ChangeCamera _charref_2 _charref_2 (Utilities|Select :Index _curentvalue :NewEnumerator0 (Math|Float|SelectFloat 2.9 1.7 (Utilities|Enum|Equal(Enum) _currentvalue "NewEnumerator4")) :NewEnumerator2 (Math|Float|SelectFloat 4.0 3.1 (Utilities|Enum|Equal(Enum) _currentvalue "NewEnumerator4")) :NewEnumerator4 (Math|Float|SelectFloat 4.0 3.1 (Utilities|Enum|Equal(Enum) _currentvalue "NewEnumerator4")) :NewEnumerator1 (Math|Float|SelectFloat 2.0 2.1 (Utilities|Enum|Equal(Enum) _currentvalue "NewEnumerator4")) :NewEnumerator3 (Math|Float|SelectFloat 4.3 2.9 (Utilities|Enum|Equal(Enum) _currentvalue "NewEnumerator4"))))
    (Transformation|DetachFromActor _charref_2 "KeepWorld" "KeepWorld" "KeepWorld")
    (else
      (return))))