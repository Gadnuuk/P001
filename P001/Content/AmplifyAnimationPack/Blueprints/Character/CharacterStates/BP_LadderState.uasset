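; Character state for climbing a BP_LadderActor, part of the Amplify Animation Pack state classes.
; On entry it shrinks the capsule, switches to Flying and aligns the character to the top or bottom entry point, using a facing dot product for top entries.
; Forward input drives climbing, while Interact locks input and applies downward force to descend.
; Each update line-traces for the ladder's ends to set the exit action through CharAnimCommunicator.
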(fn EnterState
  (params (prevStateClass :type BP%20Character%20State%20Base%20Class%20Reference))
  (bind _charref (Variables|Default|GetcharRef))
  (bind _charref_2 (Variables|Default|GetcharRef))
  (bind _charref_3 (Variables|Default|GetcharRef))
  (bind _returnvalue (Transformation|GetActorLocation _charref))
  (bind _charanimcommunicator (Variables|/Game/AmplifyAnimationPack/Blueprints/Character/BP_Character.BP_Character_C|GetcharAnimCommunicator _charref_2))
  (|CallParentFunction 0)
  (Default|SetNewCapsuleRadius _charref_3 1e+01 0.0)
  (Pawn|Components|CharacterMovement|SetMovementMode (Variables|/Script/Engine.Character|GetCharacterMovement _charref_3) "MOVE_Flying" 0)
  (bind _asbp_ladder_actor (Utilities|Casting|CastToBP_LadderActor (Variables|/Game/AmplifyAnimationPack/Blueprints/Character/BP_Character.BP_Character_C|GetobjectToInteract _charref_3)))
  (bind _currentval (Default|SetLadderActionVal _charanimcommunicator (select (Variables|/Game/AmplifyAnimationPack/Blueprints/Character/BP_Character.BP_Character_C|GetladderCanGoUp (Variables|Default|GetcharRef)) "NewEnumerator8" "NewEnumerator1")))
  (bind _willrotatetowards (CallFunction|LadderEnterGoingDownCheckAngle _currentval))
  (bind _curentvalue (Default|GetLadderActionVal _charanimcommunicator))
  (Default|SetMovementStateVal _charanimcommunicator "NewEnumerator24")
  (Default|AdjustPosition _charref _returnvalue (- (Math|Vector|SelectVector (Transformation|GetWorldLocation (Variables|/Game/AmplifyAnimationPack/Blueprints/Interactables/BP_LadderActor.BP_LadderActor_C|GetPlayerPos_GoUp _asbp_ladder_actor)) (Math|Vector|SelectVector (Transformation|GetWorldLocation (Variables|/Game/AmplifyAnimationPack/Blueprints/Interactables/BP_LadderActor.BP_LadderActor_C|GetPlayerPos_GoDown_Back _asbp_ladder_actor)) (Transformation|GetWorldLocation (Variables|/Game/AmplifyAnimationPack/Blueprints/Interactables/BP_LadderActor.BP_LadderActor_C|GetPlayerPos_GoDown _asbp_ladder_actor)) (Utilities|Enum|Equal(Enum) _curentvalue "NewEnumerator9")) (Variables|/Game/AmplifyAnimationPack/Blueprints/Character/BP_Character.BP_Character_C|GetladderCanGoUp (Variables|Default|GetcharRef))) _returnvalue) false true true)
  (Default|AdjustRotation _charref (* (Variables|/Game/AmplifyAnimationPack/Blueprints/Character/BP_Character.BP_Character_C|GetobjToInteractRotVector _charref) (Math|Float|SelectFloat -1.0 1.0 _willrotatetowards)) false 2e+01)
  (Default|SetSpeedVal (Variables|/Game/AmplifyAnimationPack/Blueprints/Character/BP_Character.BP_Character_C|GetcharAnimCommunicator _charref) 0.0))

(fn InputMoveForward
  (params (inputVal :type Float%20%28single-precision%29))
  (bind _charref (Variables|Default|GetcharRef))
  (bind _charanimcommunicator (Variables|/Game/AmplifyAnimationPack/Blueprints/Character/BP_Character.BP_Character_C|GetcharAnimCommunicator _charref))
  (|CallParentFunction 0.0)
  (if (Variables|Default|GetcanMove)
    (bind _output_get (Variables|/Game/AmplifyAnimationPack/Blueprints/Character/BP_Character.BP_Character_C|SetInputForward _charref inputVal))
    (bind _currentval (Default|SetInputFwdVal _charanimcommunicator _output_get))
    (if (!= _currentval 0.0)
      (Default|SetLadderActionVal _charanimcommunicator "NewEnumerator3"))
    (else
      (return))))

(fn InputInteract
  (|CallParentFunction)
  (if (Variables|Default|GetcanMove)
    (Default|SetLadderActionVal (Variables|/Game/AmplifyAnimationPack/Blueprints/Character/BP_Character.BP_Character_C|GetcharAnimCommunicator (Variables|Default|GetcharRef)) "NewEnumerator4")
    (Variables|Default|SetcanMove false)))

(fn UpdateState
  (params (deltaTime :type Float%20%28single-precision%29))
  (bind _charref (Variables|Default|GetcharRef))
  (bind _charref_2 (Variables|Default|GetcharRef))
  (bind _charanimcommunicator (Variables|/Game/AmplifyAnimationPack/Blueprints/Character/BP_Character.BP_Character_C|GetcharAnimCommunicator _charref))
  (|CallParentFunction 0.0)
  (bind _curentvalue (Default|GetLadderActionVal (Variables|/Game/AmplifyAnimationPack/Blueprints/Character/BP_Character.BP_Character_C|GetcharAnimCommunicator _charref_2)))
  (if (Utilities|Enum|Equal(Enum) _curentvalue "NewEnumerator3")
    (if (> (Math|Float|Sign(Float) (.z (Pawn|Components|CharacterMovement|GetLastUpdateVelocity (Variables|/Script/Engine.Character|GetCharacterMovement _charref_2)))) 0.0)
      (bind _ishitting (Default|LadderLinetraceMovementUp _charref))
      (if (not _ishitting)
        (Default|SetLadderActionVal _charanimcommunicator "NewEnumerator6")
        (Variables|Default|SetcanMove false :!label _label))
      (else
        (bind _isgrounded (Default|LadderLinetraceMovementDown _charref (Math|Float|SelectFloat -62.0 -72.0 (Utilities|Enum|Equal(Enum) _curentvalue "NewEnumerator4")) :!label _label_2))
        (if _isgrounded
          (Default|SetLadderActionVal _charanimcommunicator "NewEnumerator2")
          (goto _label))))
    (elif (Utilities|Enum|Equal(Enum) _curentvalue "NewEnumerator4")
      (Physics|AddForce (Variables|/Script/Engine.Character|GetCharacterMovement (Variables|Default|GetcharRef)) "0, 0,-100000.000000")
      (goto _label_2))))

(fn ExitState
  (|CallParentFunction)
  (Collision|SetCollisionEnabled (Variables|/Script/Engine.Character|GetCapsuleComponent (Variables|Default|GetcharRef)) "QueryAndPhysics"))

(fn LadderEnterGoingDownCheckAngle
  (params (LadderActionToCheck :type Character_LadderActions_Enum%20Enum :default "NewEnumerator0"))
  (bind _charref (Variables|Default|GetcharRef))
  (if (Utilities|Enum|Equal(Enum) LadderActionToCheck "NewEnumerator1")
    (bind _asbp_ladder_actor (Utilities|Casting|CastToBP_LadderActor (Variables|/Game/AmplifyAnimationPack/Blueprints/Character/BP_Character.BP_Character_C|GetobjectToInteract _charref)))
    (if (< (Math|Vector|DotProduct (Transformation|GetActorForwardVector _charref) (Transformation|GetActorForwardVector _asbp_ladder_actor)) 0.0)
      (Default|SetLadderActionVal (Variables|/Game/AmplifyAnimationPack/Blueprints/Character/BP_Character.BP_Character_C|GetcharAnimCommunicator (Variables|Default|GetcharRef)) "NewEnumerator9"))
    (return (< (Math|Vector|DotProduct (Transformation|GetActorForwardVector _charref) (Transformation|GetActorForwardVector _asbp_ladder_actor)) 0.0))
    (else
      (return true))))