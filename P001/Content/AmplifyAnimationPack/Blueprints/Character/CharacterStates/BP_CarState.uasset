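; Character state for using a BP_CarVehicle, covering getting in and interacting to get out.
; Entering aligns the character to the left or right entry point, sets car animation values, ignores vehicle collision, blends the camera to the car and enables its physics.
; Interact, gated on the current car action, changes that action, returns the camera, detaches the character and re-enables capsule collision.
; Exiting the state restores vehicle blocking and camera-arm collision and stops car physics.
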(fn InputInteract
  (bind _charref (Variables|Default|GetcharRef))
  (bind _charref_2 (Variables|Default|GetcharRef))
  (bind _charanimcommunicator (Variables|/Game/AmplifyAnimationPack/Blueprints/Character/BP_Character.BP_Character_C|GetcharAnimCommunicator _charref))
  (|CallParentFunction)
  (bind _curentvalue (Default|GetCarActionVal _charanimcommunicator))
  (if (Utilities|Enum|Equal(Enum) _curentvalue "NewEnumerator0")
    (Default|SetCarActionVal _charanimcommunicator "NewEnumerator11")
    (Default|ChangeCamera _charref_2 _charref_2 1.0)
    (Transformation|DetachFromActor _charref_2 "KeepWorld" "KeepWorld" "KeepWorld")
    (Collision|SetCollisionEnabled (Variables|/Script/Engine.Character|GetCapsuleComponent _charref_2) "QueryAndPhysics")
    (else
      (return))))

(fn EnterState
  (params (prevStateClass :type BP%20Character%20State%20Base%20Class%20Reference))
  (bind _charref (Variables|Default|GetcharRef))
  (bind _charref_2 (Variables|Default|GetcharRef))
  (bind _returnvalue (Transformation|GetActorLocation _charref))
  (bind _charanimcommunicator (Variables|/Game/AmplifyAnimationPack/Blueprints/Character/BP_Character.BP_Character_C|GetcharAnimCommunicator _charref))
  (|CallParentFunction 0)
  (bind _asbp_car_vehicle (Utilities|Casting|CastToBP_CarVehicle (Variables|/Game/AmplifyAnimationPack/Blueprints/Character/BP_Character.BP_Character_C|GetobjectToInteract (Variables|Default|GetcharRef))))
  (Variables|Default|SetcarActor _asbp_car_vehicle)
  (bind _curentvalue (Default|GetCarDirVal _charanimcommunicator))
  (Default|SetSpeedVal _charanimcommunicator 0.0)
  (Default|SetMovementStateVal _charanimcommunicator "NewEnumerator25")
  (Default|SetCarActionVal _charanimcommunicator "NewEnumerator10")
  (Default|AdjustPosition (Variables|Default|GetcharRef) _returnvalue (- (Transformation|GetWorldLocation (Utilities|Select :Index _curentvalue :NewEnumerator12 (Variables|/Game/AmplifyAnimationPack/Blueprints/Interactables/Car/BP_CarVehicle.BP_CarVehicle_C|GetEnterPoint_Right (Variables|Default|GetcarActor)) :NewEnumerator13 (Variables|/Game/AmplifyAnimationPack/Blueprints/Interactables/Car/BP_CarVehicle.BP_CarVehicle_C|GetEnterPoint_Left (Variables|Default|GetcarActor)))) _returnvalue) false false true)
  (Default|AdjustRotation _charref_2 (Math|Rotator|GetRotationXVector (Transformation|GetWorldRotation (Utilities|Select :Index _curentvalue :NewEnumerator12 (Variables|/Game/AmplifyAnimationPack/Blueprints/Interactables/Car/BP_CarVehicle.BP_CarVehicle_C|GetEnterPoint_Right (Variables|Default|GetcarActor)) :NewEnumerator13 (Variables|/Game/AmplifyAnimationPack/Blueprints/Interactables/Car/BP_CarVehicle.BP_CarVehicle_C|GetEnterPoint_Left (Variables|Default|GetcarActor))))) false 0.0)
  (Collision|SetCollisionResponsetoChannel (Variables|/Script/Engine.Character|GetCapsuleComponent _charref_2) "ECC_Vehicle" "ECR_Ignore")
  (Variables|/Script/Engine.SpringArmComponent|SetbDoCollisionTest (Variables|/Game/AmplifyAnimationPack/Blueprints/Character/BP_Character.BP_Character_C|GetCameraArm _charref_2) false)
  (Default|ChangeCamera (Variables|Default|GetcharRef) (Variables|Default|GetcarActor) 2.0)
  (Physics|SetSimulatePhysics (Variables|/Script/PhysXVehicles.WheeledVehicle|GetMesh (Variables|Default|GetcarActor)) true))

(fn ExitState
  (bind _charref (Variables|Default|GetcharRef))
  (|CallParentFunction)
  (Collision|SetCollisionResponsetoChannel (Variables|/Script/Engine.Character|GetCapsuleComponent _charref) "ECC_Vehicle" "ECR_Block")
  (Variables|/Script/Engine.SpringArmComponent|SetbDoCollisionTest (Variables|/Game/AmplifyAnimationPack/Blueprints/Character/BP_Character.BP_Character_C|GetCameraArm _charref) true)
  (Physics|SetSimulatePhysics (Variables|/Script/PhysXVehicles.WheeledVehicle|GetMesh (Variables|Default|GetcarActor)) false))