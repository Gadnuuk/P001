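; Arrow projectile actor for the bow weapon, launched and moved by physics simulation.
; FireArrow enables physics on the static mesh, applies a velocity-change impulse along the given direction with a slight upward boost, and rotates the actor to match.
; Each tick, pitch follows the velocity vector so the arrow tilts along its arc.
; On hit, it stops ticking and disables hit notifications and the hitbox collision.
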(event OnComponentHit(StaticMesh)
  (params (HitComponent :type Primitive%20Component%20Object%20Reference) (OtherActor :type Actor%20Object%20Reference) (OtherComp :type Primitive%20Component%20Object%20Reference) (NormalImpulse :type Vector :default "0, 0, 0") (Hit :type Hit%20Result%20Structure%20%28by%20ref%29))
  (Actor|Tick|SetActorTickEnabled false)
  (Class|PrimitiveComponent|SetNotifyRigidBodyCollision (Variables|Default|GetStaticMesh) false)
  (Collision|SetCollisionEnabled (Variables|Default|GetHitbox) "NoCollision"))

(event Custom|FireArrow
  (params (directionToAddImpulse :type Vector))
  (bind _returnvalue (* directionToAddImpulse 2e+03))
  (bind _returnvalue_2 (Transformation|GetActorUpVector))
  (bind _staticmesh (Variables|Default|GetStaticMesh))
  (bind _returnvalue_3 (* _returnvalue_2 1e+02))
  (bind _returnvalue_4 (+ _returnvalue _returnvalue_3))
  (Physics|SetSimulatePhysics _staticmesh true)
  (Physics|AddImpulse _staticmesh _returnvalue_4 "None" true)
  (Transformation|SetActorRotation (Math|Conversions|RotationFromXVector _returnvalue_4)))

(event EventTick
  (params (DeltaSeconds :type Float%20%28single-precision%29))
  (bind _returnvalue (Transformation|GetActorRotation))
  ;[1 1 1] Tick event
  (Transformation|SetActorRotation (Math|Rotator|MakeRotator (.roll _returnvalue) (.pitch (Math|Conversions|RotationFromXVector (Transformation|GetVelocity))) (.yaw _returnvalue))))

(fn ConstructionScript)