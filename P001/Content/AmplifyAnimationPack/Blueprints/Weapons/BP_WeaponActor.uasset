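; Base weapon actor that a player picks up through Interact, storing it on the character and setting a pick-up direction for animation.
; Fire and attach/detach events are empty stubs.
; Helpers spawn Niagara muzzle effects and line trace along vectors from a helper containing camera-versus-actor selection based on aiming and shootable direction.
; Trace hits spawn impact effects and blow up BP_HittableActor targets.
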(event Custom|WeaponAttached%20Event
  ;[1 1 1] Attachment custom events
)

(event Custom|WeaponUnattached%20Event
  ;[1 1 1] Attachment custom events
)

(event EventInteract
  (params (player :type BP%20Character%20Object%20Reference))
  (bind _wassuccessful (Default|WeaponStoreWeapon player self))
  (if _wassuccessful
    (|CallParentFunction player)
    (Default|SetPickObjDirVal (Variables|/Game/AmplifyAnimationPack/Blueprints/Character/BP_Character.BP_Character_C|GetcharAnimCommunicator player) "NewEnumerator2")))

(fn ConstructionScript)

(fn WeaponFire
  (params (weaponOwner :type BP%20Character%20Object%20Reference)))

(fn WeaponMuzzleEffect
  (Niagara|SpawnSystematLocation (Variables|FiringVariables|GetMuzzleEffect) (Transformation|GetSocketLocation (Variables|Default|GetMesh) "muzzleSocket") "0, 0, 0" "1.000000,1.000000,1.000000" true true "AutoRelease"))

(fn WeaponLinetraceShot
  (params (ownerRef :type BP%20Character%20Object%20Reference))
  (bind _curentvalue (Default|GetCanShootinDirectionVal (Variables|/Game/AmplifyAnimationPack/Blueprints/Character/BP_Character.BP_Character_C|GetcharAnimCommunicator ownerRef)))
  (bind (_outhit _returnvalue) (Collision|LineTraceForObjects (.start (Utilities|WeaponDecideLinetraceVectors ownerRef _curentvalue)) (+ (.start (Utilities|WeaponDecideLinetraceVectors ownerRef _curentvalue)) (* (.dir (Utilities|WeaponDecideLinetraceVectors ownerRef _curentvalue)) (Variables|FiringVariables|GetBulletRange))) (Utilities|Array|MakeArray "ObjectTypeQuery1" "ObjectTypeQuery2") false 0 "None"))
  (if _returnvalue
    (Niagara|SpawnSystematLocation "/Game/Assets/AmplifyAnimationPack/FX/NS_ImpactFX.NS_ImpactFX" (.Location (Collision|BreakHitResult _outhit)) "0, 0, 0" "1.000000,1.000000,1.000000" true true "AutoRelease")
    (bind _asbp_hittable_actor (Utilities|Casting|CastToBP_HittableActor (.HitActor (Collision|BreakHitResult _outhit))))
    (Default|HittableBlowUp _asbp_hittable_actor)))